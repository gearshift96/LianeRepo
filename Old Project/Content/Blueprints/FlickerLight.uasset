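; FlickerLight is an actor whose point light flickers once when another actor first overlaps it, then stays lit.
; The overlap event sets a FlickerOn flag, which Tick polls every frame.
; A DoOnce gate with no reset runs a hard-coded chain of short delays that alternates the light intensity between bright and off, ending bright.
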(event `self.ReceiveBeginPlay`)

(event `self.ReceiveActorBeginOverlap`
  (params (OtherActor :type "Actor Object Reference"))
  (set `self.FlickerOn` true))

(event `self.ReceiveTick`
  (params (DeltaSeconds :type "Float (single-precision)"))
  (if (`self.FlickerOn`)
    (`/Engine/EditorBlueprintResources/StandardMacros.DoOnce` false
      (:`Completed`
        (`KismetSystemLibrary.Delay` 0.1)
        (`LightComponent.SetIntensity` (`self.PointLight`) 1300.0)
        (`KismetSystemLibrary.Delay` 0.1)
        (`LightComponent.SetIntensity` (`self.PointLight`) 0.0)
        (`KismetSystemLibrary.Delay` 0.1)
        (`LightComponent.SetIntensity` (`self.PointLight`) 1300.0)
        (`KismetSystemLibrary.Delay` 0.1)
        (`LightComponent.SetIntensity` (`self.PointLight`) 0.0)
        (`KismetSystemLibrary.Delay` 0.1)
        (`LightComponent.SetIntensity` (`self.PointLight`) 1300.0)
        (`KismetSystemLibrary.Delay` 0.1)
        (`LightComponent.SetIntensity` (`self.PointLight`) 0.0)
        (`KismetSystemLibrary.Delay` 0.1)
        (`LightComponent.SetIntensity` (`self.PointLight`) 1300.0)))))

(fn `UserConstructionScript`)