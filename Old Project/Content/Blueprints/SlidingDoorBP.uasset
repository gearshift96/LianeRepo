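; Sliding door actor that instantly shifts its Door component out of the way, once, when ShouldOpen is set.
; Tick polls ShouldOpen and HasOpened, then calls OpenDoor.
; OpenDoor doubles the box extent of the whole actor's bounds and moves the door that far in the negative world direction of the first enabled axis flag, checking X, Y, then Z.
; Nothing here closes it or sets ShouldOpen.
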(event `Check ShouldOpen`
  ;[1 1 1] Open the door when needed
  (if (`self.ShouldOpen`)
    (if (not (`self.HasOpened`))
      (`self.OpenDoor`))))

(event `self.ReceiveTick`
  (params (DeltaSeconds :type "Float (single-precision)"))
  ;[1 1 1] Check if door should open
  (`self.Check ShouldOpen`))

(event `OpenDoor`
  ;[1 1 1] Logic for opening the door.
  ;;[1 1 1] Get size of current door (It's only half size)
  (bind (_center _boxextent) (`GameplayStatics.GetActorArrayBounds` (`|MakeArray` self))) ; Box extent only gets half the size
  (set `self.SizeOfCube` _boxextent)
  ;;[1 0 0] Check if door should open on the X axis.
  (if (`self.OpenX`)
    (`SceneComponent.K2_SetWorldLocation` (`self.Door`) (`KismetMathLibrary.MakeVector` (- (.x (`SceneComponent.K2_GetComponentLocation` (`self.Door`))) (* (.x (`self.SizeOfCube`)) 2.0)) (.y (`SceneComponent.K2_GetComponentLocation` (`self.Door`))) (.z (`SceneComponent.K2_GetComponentLocation` (`self.Door`)))) false false)
    (set `self.HasOpened` true)
    (else
      ;;[0.1535 1 0] Check if door should open on the Y axis.
      (if (`self.OpenY`)
        (`SceneComponent.K2_SetWorldLocation` (`self.Door`) (`KismetMathLibrary.MakeVector` (.x (`SceneComponent.K2_GetComponentLocation` (`self.Door`))) (- (.y (`SceneComponent.K2_GetComponentLocation` (`self.Door`))) (* (.y (`self.SizeOfCube`)) 2.0)) (.z (`SceneComponent.K2_GetComponentLocation` (`self.Door`)))) false false)
        (set `self.HasOpened` true)
        (else
          ;;[0.07847 0 1] Check if door should open on the Z axis
          (if (`self.OpenZ`)
            (`SceneComponent.K2_SetWorldLocation` (`self.Door`) (`KismetMathLibrary.MakeVector` (.x (`SceneComponent.K2_GetComponentLocation` (`self.Door`))) (.y (`SceneComponent.K2_GetComponentLocation` (`self.Door`))) (- (.z (`SceneComponent.K2_GetComponentLocation` (`self.Door`))) (* (.z (`self.SizeOfCube`)) 2.0))) false false)
            (set `self.HasOpened` true)))))))

(fn `UserConstructionScript`)