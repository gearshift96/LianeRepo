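; BP_PhotoModeManager switches the player in and out of photo mode, acting on its owning PlayerController.
; Activation spawns or reuses a BP_PhotoPawn offset from the controlled pawn, turns it toward that pawn and possesses it.
; It sets global time dilation to zero and offsets this with a huge custom dilation on the photo pawn.
; Deactivation is delegated to the photo pawn, and enter and exit dispatchers announce both transitions.
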(event `ActivatePhotoMode`
  (bind _returnvalue (`Controller.K2_GetPawn` (cast `PlayerController` (`self.GetOwner`) :!pure true)))
  (bind _returnvalue_2 (`KismetMathLibrary.MakeTransform` (`KismetMathLibrary.MakeVector` (- (.x (.location (`Actor.GetTransform` (`Controller.K2_GetPawn` (cast `PlayerController` (`self.GetOwner`) :!pure true))))) 200.0) (.y (.location (`Actor.GetTransform` (`Controller.K2_GetPawn` (cast `PlayerController` (`self.GetOwner`) :!pure true))))) (+ (.z (.location (`Actor.GetTransform` (`Controller.K2_GetPawn` (cast `PlayerController` (`self.GetOwner`) :!pure true))))) 50.0)) (.rotation (`Actor.GetTransform` (`Controller.K2_GetPawn` (cast `PlayerController` (`self.GetOwner`) :!pure true)))) (.scale (`Actor.GetTransform` (`Controller.K2_GetPawn` (cast `PlayerController` (`self.GetOwner`) :!pure true))))))
  ;[1 1 1] Possess Photo Pawn and stop time
  (`/Engine/EditorBlueprintResources/StandardMacros.IsValid` (`self.PhotoPawn`)
    (:`Is Valid`
      (`Actor.K2_SetActorTransform` (`self.PhotoPawn`) _returnvalue_2 false true))
    (:`Is Not Valid`
      (bind _returnvalue_3 (`|SpawnActorFromClass` "/Game/PhotoMode/Blueprints/BP_PhotoPawn.BP_PhotoPawn_C" _returnvalue_2 "Undefined" "OverrideRootScale"))
      (bind _output_get (set `self.PhotoPawn` _returnvalue_3))
      (set `/Game/PhotoMode/Blueprints/BP_PhotoPawn.OwnerPawn` _returnvalue _output_get)))
  (`Actor.K2_SetActorRotation` (`self.PhotoPawn`) (`KismetMathLibrary.FindLookAtRotation` (`Actor.K2_GetActorLocation` (`self.PhotoPawn`)) (`Actor.K2_GetActorLocation` _returnvalue)) false)
  (`Controller.Possess` (cast `PlayerController` (`self.GetOwner`) :!pure true) (`self.PhotoPawn`))
  (`GameplayStatics.SetGlobalTimeDilation` 1e-07)
  (set `Actor.CustomTimeDilation` 10000.0 (`self.PhotoPawn`))
  (set `self.IsModeActive` true)
  (`self.OnEnterPhotoModeDispatcher`))

(event `DeactivatePhotoMode`
  ;[1 1 1] Deactivate Photo Mode
  (`/Engine/EditorBlueprintResources/StandardMacros.IsValid` (`self.PhotoPawn`)
    (:`Is Valid`
      (`/Game/PhotoMode/Blueprints/BP_PhotoPawn.DeactivatePhotoMode` (`self.PhotoPawn`))
      (`self.OnExitPhotoModeDispatcher`))))