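; PlayerState component for match lobby members, tracking ready status, map vote and scoreboard visibility.
; On BeginPlay it creates lobby and scoreboard widgets for the local player, printing an error if the owner isn't a PlayerState.
; Server events forward ready requests and vote tally updates to the GameState's BP_LobbyManagerComponent.
; Votes apply locally before reaching the server; RepNotifies broadcast ready and vote changes and apply server-forced scoreboard display.
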(event `self.ReceiveBeginPlay`
  ;[1 1 1] Create Lobby Widget on local player
  (bind _asplayer_state (cast `PlayerState` (`self.GetOwner`))
    (:`then`
      (bind _asplayer_controller (cast `PlayerController` (`Actor.GetOwner` _asplayer_state)))
      (if (`Controller.IsLocalPlayerController` _asplayer_controller)
        (bind _returnvalue (`|CreateWidget` "/Game/GenericShooter/Addons/MatchLobby/Core/UI/Lobby/WBP_Lobby.WBP_Lobby_C" _asplayer_controller (cast `PlayerState` (`self.GetOwner`) :!pure true)))
        (`UserWidget.AddToPlayerScreen` _returnvalue 0)
        (bind _returnvalue_2 (`|CreateWidget` "/Game/GenericShooter/Addons/MatchLobby/Core/UI/Scoreboard/WBP_Scoreboard.WBP_Scoreboard_C" _asplayer_controller))
        (bind _output_get (set `self.ScoreboardWidget` _returnvalue_2))
        (`Widget.SetVisibility` _output_get "Collapsed")
        (`UserWidget.AddToPlayerScreen` _returnvalue_2 0)))
    (:`CastFailed`
      (`KismetSystemLibrary.PrintString` "ERROR: BP_LOBBYMEMBERCOMPONENT CREATED INSIDE A NON-PLAYERSTATE CLASS. PLEASE DO NOT DO THIS." true true (struct :`R` 1.0 :`G` 0.053367 :`A` 1.0) 20.0))))

(event `VoteForMapIndex`
  (params (DesiredMapVoteIndex :type Integer))
  ;[1 1 1] Networking for map voting
  (bind _output_get (set `self.MapVoteIndex` DesiredMapVoteIndex))
  (`self.ServerVoteForMapIndex` _output_get)
  (`self.OnMapVoteIndexChanged` _output_get))

(event `ServerRequestReadyStatusChange`
  (params (bReady :type Boolean))
  ;[1 1 1] Networking functions to handle requesting readying of a player
  (`/Game/GenericShooter/Addons/MatchLobby/Core/BP_LobbyManagerComponent.RequestReadyStatusChange` (`Actor.GetComponentByClass` (`GameplayStatics.GetGameState`) "/Game/GenericShooter/Addons/MatchLobby/Core/BP_LobbyManagerComponent.BP_LobbyManagerComponent_C") (cast `PlayerState` (`self.GetOwner`) :!pure true) bReady))

(event `ServerVoteForMapIndex`
  (params (DesiredMapVoteIndex :type Integer))
  ;[1 1 1] Networking for map voting
  (set `self.MapVoteIndex` DesiredMapVoteIndex)
  (`/Game/GenericShooter/Addons/MatchLobby/Core/BP_LobbyManagerComponent.UpdateMapVoteTotals` (`Actor.GetComponentByClass` (`GameplayStatics.GetGameState`) "/Game/GenericShooter/Addons/MatchLobby/Core/BP_LobbyManagerComponent.BP_LobbyManagerComponent_C")))

(event `ServerClearMapVote`
  ;[1 1 1] Networking for map voting
  (`self.ClearMapVote`))

(event `ServerRequestToggleReadyStatus`
  ;[1 1 1] Networking functions to handle requesting readying of a player
  (`self.ServerRequestReadyStatusChange` (not (`self.IsReady`))))

(fn `ClearMapVote`
  (set `self.MapVoteIndex` -1)
  (if (`KismetSystemLibrary.IsServer`)
    (return)
    (else
      (`self.ServerClearMapVote`)
      (return))))

(fn `IsReady`
  (returns (bReady :type Boolean))
  (return (`self.bReady`)))

(fn `OnRep_bForceShowScoreboard`
  (`self.SetScoreboardVisibility` (`self.bForceShowScoreboard`))
  (return))

(fn `OnRep_bReady`
  (`self.OnReadyStatusChanged` (`self.bReady`))
  (return))

(fn `OnRep_MapVoteIndex`
  (`self.OnMapVoteIndexChanged` (`self.MapVoteIndex`))
  (return))

(fn `SetReady`
  (params (bNewReady :type Boolean))
  (if (`KismetSystemLibrary.IsServer`)
    (set `self.bReady` bNewReady)
    (return)
    (else
      (return))))

(fn `SetScoreboardVisibility`
  (params (bVisible :type Boolean))
  (`self.ScoreboardWidget`
    (:`then`
      (`Widget.SetVisibility` (`self.ScoreboardWidget`) (select `bool` (or bVisible (`self.bForceShowScoreboard`)) :`false` "Collapsed" :`true` "HitTestInvisible" :!type "ESlateVisibility Enum"))
      (`self.OnScoreboardVisbilityChanged` (`local.bVisible`))
      (return))
    (:`else`
      (return))))

(fn `ToggleScoreboardVisibility`
  (bind _scoreboardwidget (`self.ScoreboardWidget`)
    (:`then`
      (`self.SetScoreboardVisibility` (not (`Widget.IsVisible` _scoreboardwidget)))
      (return))
    (:`else`
      (return))))