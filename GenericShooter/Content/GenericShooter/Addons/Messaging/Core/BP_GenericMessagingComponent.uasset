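; Player Controller component that delivers class-based local messages to players in the generic shooter messaging addon, destroying itself on any other owner.
; ClientReceiveLocalMessage skips dedicated servers, constructs the message class, runs its ClientReceive and optionally notifies listeners via OnMessageReceived.
; ServerBroadcastMessage relays messages to controllers through the GameState PlayerArray, only for classes whose defaults permit client broadcasting.
; It also wraps SpawnSound2D as a helper.
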(event `self.ReceiveBeginPlay`
  (`self.WarnAndDestroyIfAddedToNonController`))

(event `ClientReceiveLocalMessage`
  (params (LocalMessage :type "/Game/GenericShooter/Addons/Messaging/Core/BP_LocalMessage Class Reference") (Switch :type Integer) (MessageString :type String) (RelatedPlayerStates :type "Array of PlayerState Object Reference") (OptionalObjects :type "Array of Object Object Reference") (OptionalClasses :type "Array of Object Class Reference"))
  (bind _fbpclientreceivedata (make `/Game/GenericShooter/Addons/Messaging/Core/FBPClientReceiveData` (cast `PlayerController` (`self.GetOwner`) :!pure true) self Switch MessageString RelatedPlayerStates OptionalObjects OptionalClasses))
  (if (not (`KismetSystemLibrary.IsDedicatedServer`))
    (`/Engine/EditorBlueprintResources/StandardMacros.IsValid` (`GameplayStatics.GetGameState`)
      (:`Is Valid`
        (bind _returnvalue (`|GenericCreateObject` LocalMessage self))
        (`/Game/GenericShooter/Addons/Messaging/Core/BP_LocalMessage.ClientReceive` _returnvalue _fbpclientreceivedata)
        (if (`/Game/GenericShooter/Addons/Messaging/Core/BP_LocalMessage.bBroadcastToMessageListeners` _returnvalue)
          (`self.OnMessageReceived` LocalMessage _fbpclientreceivedata))))))

(event `ServerBroadcastMessage`
  (params (LocalMessage :type "/Game/GenericShooter/Addons/Messaging/Core/BP_LocalMessage Class Reference") (Switch :type Integer) (MessageString :type String) (RelatedPlayerStates :type "Array of PlayerState Object Reference") (OptionalObject :type "Array of Object Object Reference") (OptionalClasses :type "Array of Object Class Reference"))
  (if (`.bCanBeBroadcastedFromClient` (defaults `/Game/GenericShooter/Addons/Messaging/Core/BP_GenericMessagingComponent` LocalMessage))
    (for _array_element (`GameStateBase.PlayerArray` (`GameplayStatics.GetGameState`))
      (bind _asplayer_controller (cast `PlayerController` (`Actor.GetOwner` _array_element)))
      (`self.ClientReceiveLocalMessage` (`Actor.GetComponentByClass` _asplayer_controller "BP_GenericMessagingComponent_C") LocalMessage Switch MessageString RelatedPlayerStates OptionalObject OptionalClasses))
    (else
      (`KismetSystemLibrary.PrintString` "ERROR: CLIENT TRIED BROADCASTING A MESSAGE IT SHOULD NEVER TRY TO BROADCAST!" true true (struct :`R` 1.0 :`A` 1.0) 10.0))))

(fn `SpawnSound2D`
  (params (Sound :type "SoundCue Object Reference") (VolumeMultiplier :type "Float (double-precision)" :default 1.0) (PitchMultiplier :type "Float (double-precision)" :default 1.0) (StartTime :type "Float (double-precision)" :default 0.0) (ConcurrencySettings :type "SoundConcurrency Object Reference") (PersistAcrossLevelTransition :type Boolean) (AutoDestroy :type Boolean :default true))
  (returns (AudioComponent :type "AudioComponent Object Reference"))
  (bind _returnvalue (`GameplayStatics.SpawnSound2D` Sound VolumeMultiplier PitchMultiplier StartTime ConcurrencySettings PersistAcrossLevelTransition AutoDestroy))
  (return _returnvalue))

(fn `WarnAndDestroyIfAddedToNonController`
  (cast `PlayerController` (`self.GetOwner`)
    (:`then`
      (return))
    (:`CastFailed`
      (`KismetSystemLibrary.PrintString` "ERROR: BP_GenericMessagingComponent is meant to be added to Player Controller classes only!" true true (struct :`R` 1.0 :`G` 0.013706 :`A` 1.0) 10.0)
      (`self.K2_DestroyComponent`)
      (return))))