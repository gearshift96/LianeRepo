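; BP_Message_Welcome is a message class that announces a player joining the game on each receiving client.
; ClientReceive takes the welcomed player from the first related player state and does nothing if none is passed.
; If that player is local, the messaging component plays a 2D welcome sound.
; Otherwise, it prints a timed, colored on-screen text naming the player who joined.
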(event `self.ClientReceive`
  (params (ClientReceiveData :type "/Game/GenericShooter/Addons/Messaging/Core/FBPClientReceiveData Structure"))
  (bind (_localpc _localmessagingcomponent _messageindex _messagestring _relatedplayerstates) (break `/Game/GenericShooter/Addons/Messaging/Core/FBPClientReceiveData` ClientReceiveData))
  (bind _output (`|GetArrayItem` _relatedplayerstates))
  ;[1 1 1] Make sure message has a valid player state passed in it, otherwise do nothing.
  (if (`KismetArrayLibrary.Array_IsValidIndex` _relatedplayerstates)
    ;[1 1 1] Is the welcomed player the local player?
    (if (== (`Controller.PlayerState` _localpc) _output)
      ;[1 1 1] If local, play the 'Welcome to Server' sound message.
      (`/Game/GenericShooter/Addons/Messaging/Core/BP_GenericMessagingComponent.SpawnSound2D` _localmessagingcomponent "/Game/GenericShooter/Addons/Messaging/Messages/Welcome/A_Welcome_Cue.A_Welcome_Cue" 1.0 1.0 0.0 null false true)
      (else
        ;[1 1 1] If welcomed player is not local, simply print a string to the screen saying that this player has joined the game.
        (`KismetSystemLibrary.PrintText` _localmessagingcomponent (`|FormatText` "{Player} has joined the game." (`KismetTextLibrary.Conv_StringToText` (`PlayerState.GetPlayerName` _output))) true true (struct :`G` 1.0 :`B` 0.075142 :`A` 1.0) 5.0)))))