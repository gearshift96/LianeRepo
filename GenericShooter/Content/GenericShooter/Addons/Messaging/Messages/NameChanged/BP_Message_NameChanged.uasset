(event `self.ClientReceive`
  (params (ClientReceiveData :type "/Game/GenericShooter/Addons/Messaging/Core/FBPClientReceiveData Structure"))
  (bind (_localpc _localmessagingcomponent _messageindex _messagestring _relatedplayerstates) (break `/Game/GenericShooter/Addons/Messaging/Core/FBPClientReceiveData` ClientReceiveData))
  (bind _output (`|GetArrayItem` _relatedplayerstates))
  (bind _returnvalue (`KismetTextLibrary.Conv_StringToText` (`PlayerState.GetPlayerName` _output)))
  ;[1 1 1] Make sure message has a valid player state passed in it, otherwise do nothing.
  (if (`KismetArrayLibrary.Array_IsValidIndex` _relatedplayerstates)
    ;[1 1 1] Is the welcomed player the local player?
    (if (== (`Controller.PlayerState` _localpc) _output)
      ;[1 1 1] If player who changed name is local, display 'You have changed' name text.
      (`KismetSystemLibrary.PrintText` _localmessagingcomponent (`|FormatText` "You have changed your name to {Player}." _returnvalue) true true (struct :`G` 1.0 :`B` 0.075142 :`A` 1.0) 5.0)
      (else
        ;[1 1 1] If welcomed player is not local, simply print a string saying someone has changed their name.
        (`KismetSystemLibrary.PrintText` _localmessagingcomponent (`|FormatText` "A player has changed their name to {Player}." _returnvalue) true true (struct :`G` 1.0 :`B` 0.075142 :`A` 1.0) 5.0)))))