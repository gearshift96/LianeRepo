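; Settings menu option that displays and changes the volume of the sound class named by its OptionID.
; On widget creation it reads that volume from the audio settings bucket via the game instance's settings manager and snaps the default percentage down to a step multiple.
; On choice change it converts the percentage to a fraction, sets and saves it in the bucket, then broadcasts the option change.
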(event `/Game/GenericShooter/Addons/MainMenu/Core/Controls/BP_DynamicMenuOption_Choice.ChoiceChanged`
  (params (ChoiceScroller :type "/Game/GenericShooter/Addons/MainMenu/Core/Controls/WBP_ChoiceScroller Object Reference") (NewChoiceIndex :type Integer))
  (bind _gameinstance (`self.GameInstance`)
    (:`then`
      (bind _settingsmanager (message `/Game/GenericShooter/Addons/SettingsManager/Core/BPI_SettingsManagerHolder.GetSettingsManager` _gameinstance))
      (bind _bucket (`/Game/GenericShooter/Addons/SettingsManager/Core/BP_SettingsManager.GetBucketByClass` _settingsmanager "/Game/GenericShooter/Addons/SettingsManager/Core/BP_SettingsBucket_Audio.BP_SettingsBucket_Audio_C"))
      (bind _asbp_settings_bucket_audio (cast `/Game/GenericShooter/Addons/SettingsManager/Core/BP_SettingsBucket_Audio` _bucket)
        (:`then`
          (bind _value (`self.GetOptionValueAsInteger`))
          (`/Game/GenericShooter/Addons/SettingsManager/Core/BP_SettingsBucket_Audio.SetVolume` _asbp_settings_bucket_audio (`self.OptionID`) (/ (`KismetMathLibrary.Conv_IntToDouble` _value) 100.0) true)
          (bind _value_2 (`self.GetOptionValueAsString`))
          (`self.OnOptionChanged` self _value_2))
        (:`CastFailed`
          (`KismetSystemLibrary.PrintString` null "ERROR: Volume option changed but failed to get audio settings bucket!"))))
    (:`else`
      (`KismetSystemLibrary.PrintString` ChoiceScroller "ERROR: Volume option changed without a game instance reference!"))))

(fn `CreateWidget`
  (params (OwningPlayerController :type "PlayerController Object Reference") (GameInstance :type "GameInstance Object Reference"))
  (returns (OptionWidget :type "UserWidget Object Reference"))
  (set `self.GameInstance` GameInstance)
  (`|ExecutionSequence`
    (:`then_0`
      (bind _gameinstance (`self.GameInstance`)
        (:`then`
          (bind _settingsmanager (message `/Game/GenericShooter/Addons/SettingsManager/Core/BPI_SettingsManagerHolder.GetSettingsManager` _gameinstance))
          (bind _bucket (`/Game/GenericShooter/Addons/SettingsManager/Core/BP_SettingsManager.GetBucketByClass` _settingsmanager "/Game/GenericShooter/Addons/SettingsManager/Core/BP_SettingsBucket_Audio.BP_SettingsBucket_Audio_C"))
          (bind _asbp_settings_bucket_audio (cast `/Game/GenericShooter/Addons/SettingsManager/Core/BP_SettingsBucket_Audio` _bucket))
          (bind _volume (`/Game/GenericShooter/Addons/SettingsManager/Core/BP_SettingsBucket_Audio.GetVolume` _asbp_settings_bucket_audio (`self.OptionID`)))
          (set `self.DefaultValue` (* (/ (`KismetMathLibrary.FTrunc` (* _volume 100.0)) (`self.Step`)) (`self.Step`))))
        (:`else`)))
    (:`then_1`
      (bind _optionwidget (`parent.CreateWidget` (`local.OwningPlayerController`) (`self.GameInstance`)))
      (return _optionwidget))))