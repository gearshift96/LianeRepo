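; Dynamic settings menu option that lets the player pick a character skin from a choice scroller.
; BuildValues fills the choices from the skin lookup DataTable, using friendly names as text and row names as tags.
; SetPreviewCharacter selects the entry matching the preview character's saved skin key, falling back to its current one.
; Changing the choice applies and saves that skin through the preview character's skinner component.
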(event `self.ChoiceChanged`
  (params (ChoiceScroller :type "/Game/GenericShooter/Addons/MainMenu/Core/Controls/WBP_ChoiceScroller Object Reference") (NewChoiceIndex :type Integer))
  (bind _previewcharacter (`self.PreviewCharacter`)
    (:`then`
      (`/Game/GenericShooter/Addons/Skinner/Core/BP_SkinnerComponent.ChangeCharacterSkin` (`/Game/GenericShooter/Addons/Skinner/Core/BP_SkinnerPreview.BP_BasicSkinnerComponent` _previewcharacter) (`KismetStringLibrary.Conv_StringToName` (`.Tag_5_761A29D4451DCE57DE275D95535F542A` (break `/Game/GenericShooter/Addons/MainMenu/Core/Controls/FTaggedText` (`|GetArrayItem` (`self.Choices`) NewChoiceIndex)))) true false))
    (:`else`)))

(fn `BuildValues`
  (returns (bBuiltValues :type Boolean))
  (`KismetArrayLibrary.Array_Clear` (`self.Choices`))
  (bind _characterskinlookuptable (`self.CharacterSkinLookupTable`)
    (:`then`
      (bind _outrownames (`DataTableFunctionLibrary.GetDataTableRowNames` _characterskinlookuptable))
      (for _array_element _outrownames
        (bind _returnvalue (`|GetDataTableRow` _characterskinlookuptable _array_element)
          (:`then`
            (`KismetArrayLibrary.Array_Add` (`self.Choices`) (make `/Game/GenericShooter/Addons/MainMenu/Core/Controls/FTaggedText` (`.UserFriendlyName_21_BF54A6664C8B7BEC427BAFBB99657ED3` (break `/Game/GenericShooter/Addons/Skinner/Core/FCharacterMeshInfo` _returnvalue)) (`KismetStringLibrary.Conv_NameToString` _array_element))))))
      (return true))
    (:`else`
      (set `self.Choices` (`|MakeArray` (make `/Game/GenericShooter/Addons/MainMenu/Core/Controls/FTaggedText` "INVALID LOOKUP TABLE")))
      (return false))))

(fn `SetPreviewCharacter`
  (params (SkinPreview :type "/Game/GenericShooter/Addons/Skinner/Core/BP_SkinnerPreview Object Reference"))
  (locals (LoadedCharacterName :type Name))
  (set `self.PreviewCharacter` SkinPreview)
  (bind _previewcharacter (`self.PreviewCharacter`)
    (:`then`
      (bind _bp_basicskinnercomponent (`/Game/GenericShooter/Addons/Skinner/Core/BP_SkinnerPreview.BP_BasicSkinnerComponent` _previewcharacter))
      (bind (_characterkeyname _bloaded) (`/Game/GenericShooter/Addons/Skinner/Core/BP_SkinnerComponent.LoadKeyName` _bp_basicskinnercomponent 0))
      (set `local.LoadedCharacterName` (select `bool` _bloaded :`false` (`/Game/GenericShooter/Addons/Skinner/Core/BP_SkinnerComponent.CharacterKeyName` _bp_basicskinnercomponent) :`true` _characterkeyname))
      (for (_array_element _array_index) (`self.Choices`)
        (if (== (`KismetStringLibrary.Conv_StringToName` (`.Tag_5_761A29D4451DCE57DE275D95535F542A` (break `/Game/GenericShooter/Addons/MainMenu/Core/Controls/FTaggedText` _array_element))) (`local.LoadedCharacterName`))
          (set `self.SelectedChoice` _array_index)
          (bind _aswbp_choice_scroller (cast `/Game/GenericShooter/Addons/MainMenu/Core/Controls/WBP_ChoiceScroller` (`self.CreatedWidget`)))
          (`/Game/GenericShooter/Addons/MainMenu/Core/Controls/WBP_ChoiceScroller.SetSelectedChoice` _aswbp_choice_scroller (`self.SelectedChoice`))))
      (return))
    (:`else`
      (return))))