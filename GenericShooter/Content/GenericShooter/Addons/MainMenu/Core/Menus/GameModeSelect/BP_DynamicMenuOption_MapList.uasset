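; Dynamic main menu option that lists the maps supporting a given game mode alias.
; BuildValues clears the choices, starts RetrieveMapChoices and returns immediately, before the async asset load completes.
; Loaded BP_MapMetaInfo_Base class defaults are filtered by GameModeAlias, adding display names tagged with map URLs.
; The first choice is then selected and the widget refreshed; the URL string getter passes through the option's string value.
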(event `RetrieveMapChoices`
  (bind _outprimaryassetidlist (`KismetSystemLibrary.GetPrimaryAssetIdList` "BP_MapMetaInfo_Base"))
  (`AsyncActionLoadPrimaryAssetList.AsyncLoadPrimaryAssetList` (`self.WorldContextObject`) _outprimaryassetidlist
    (:`then`
      (for _array_element _outprimaryassetidlist
        (bind _asbp_map_meta_info_base (castclass `/Game/GenericShooter/Addons/MatchLobby/Core/BP_MapMetaInfo_Base` (`KismetSystemLibrary.GetClassFromPrimaryAssetId` _array_element)))
        (bind (_mapdisplayname _url _voteimage _supportedgamemodealiases) (defaults `/Game/GenericShooter/Addons/MainMenu/Core/Menus/GameModeSelect/BP_DynamicMenuOption_MapList` _asbp_map_meta_info_base))
        (if (`KismetArrayLibrary.Array_Contains` _supportedgamemodealiases (`self.GameModeAlias`))
          (`KismetArrayLibrary.Array_Add` (`self.Choices`) (make `/Game/GenericShooter/Addons/MainMenu/Core/Controls/FTaggedText` _mapdisplayname (`KismetStringLibrary.Conv_NameToString` _url)))))
      (set `self.SelectedChoice` 0)
      (`self.ForceUpdateWidgetValues`))))

(fn `BuildValues`
  (returns (bBuiltValues :type Boolean))
  (`KismetArrayLibrary.Array_Clear` (`self.Choices`))
  (`self.RetrieveMapChoices`)
  (return true))

(fn `GetOptionValueAsURLString`
  (returns (URLString :type String))
  (bind _value (`self.GetOptionValueAsString`))
  (return _value))