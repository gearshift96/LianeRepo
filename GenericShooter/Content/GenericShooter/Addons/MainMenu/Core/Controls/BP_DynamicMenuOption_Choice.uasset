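; Menu option object for the main menu that presents a list of tagged text choices as a choice scroller widget.
; CreateWidget builds the values, optionally uppercases title and choices, then constructs a WBP_ChoiceScroller and binds its change event.
; Getters read the scroller's selected tag, text or index, and format an OptionID=value URL string.
; Selection changes fire OnOptionChanged, while ForceUpdateWidgetValues pushes choices back without firing it.
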(event `self.ForceUpdateWidgetValues`
  (`self.ForceUppercaseChoices`)
  (bind _aswbp_choice_scroller (cast `/Game/GenericShooter/Addons/MainMenu/Core/Controls/WBP_ChoiceScroller` (`self.CreatedWidget`)))
  (`/Game/GenericShooter/Addons/MainMenu/Core/Controls/WBP_ChoiceScroller.SetChoices` _aswbp_choice_scroller (`self.Choices`) (`self.SelectedChoice`) false))

(fn `ChoiceChanged`
  (params (ChoiceScroller :type "/Game/GenericShooter/Addons/MainMenu/Core/Controls/WBP_ChoiceScroller Object Reference") (NewChoiceIndex :type Integer))
  (bind _value (`self.GetOptionValueAsString`))
  (`self.OnOptionChanged` self _value)
  (return))

(fn `CreateWidget`
  (params (OwningPlayerController :type "PlayerController Object Reference") (GameInstance :type "GameInstance Object Reference"))
  (returns (OptionWidget :type "UserWidget Object Reference"))
  (bind _optiontitle (`self.OptionTitle`))
  (`self.BuildValues`)
  (`self.ForceUppercaseChoices`)
  (bind _returnvalue (`|GenericCreateObject` "/Game/GenericShooter/Addons/MainMenu/Core/Controls/WBP_ChoiceScroller.WBP_ChoiceScroller_C" self (select `bool` (`self.bForceUppercase`) :`false` _optiontitle :`true` (`KismetTextLibrary.TextToUpper` _optiontitle)) (`self.Choices`) (`self.SelectedChoice`)))
  (add `/Game/GenericShooter/Addons/MainMenu/Core/Controls/WBP_ChoiceScroller.OnChoiceChanged` _returnvalue (`|CreateDelegate` :!event `ChoiceChanged`))
  (`UserWidget.SetOwningPlayer` _returnvalue OwningPlayerController)
  (bind _output_get (set `self.CreatedWidget` _returnvalue))
  (return _output_get))

(fn `ForceUppercaseChoices`
  (bind _choices (`self.Choices`))
  (if (`self.bForceUppercase`)
    (for (_array_element _array_index) _choices
      (bind (_text _tag) (break `/Game/GenericShooter/Addons/MainMenu/Core/Controls/FTaggedText` _array_element))
      (`KismetArrayLibrary.Array_Set` _choices _array_index (make `/Game/GenericShooter/Addons/MainMenu/Core/Controls/FTaggedText` (`KismetTextLibrary.TextToUpper` _text) _tag)))
    (return)
    (else
      (return))))

(fn `GetOptionDisplayText`
  (returns (DisplayText :type Text))
  (bind _createdwidget (`self.CreatedWidget`)
    (:`then`
      (bind _aswbp_choice_scroller (cast `/Game/GenericShooter/Addons/MainMenu/Core/Controls/WBP_ChoiceScroller` _createdwidget)
        (:`then`
          (return (`/Game/GenericShooter/Addons/MainMenu/Core/Controls/WBP_ChoiceScroller.GetSelectedChoiceText` _aswbp_choice_scroller)))
        (:`CastFailed`
          _)))
    (:`else`
      _))
  (return ""))

(fn `GetOptionSelectedIndex`
  (returns (SelectedIndex :type Integer))
  (bind _createdwidget (`self.CreatedWidget`)
    (:`then`
      (bind _aswbp_choice_scroller (cast `/Game/GenericShooter/Addons/MainMenu/Core/Controls/WBP_ChoiceScroller` _createdwidget)
        (:`then`
          (return (`/Game/GenericShooter/Addons/MainMenu/Core/Controls/WBP_ChoiceScroller.GetSelectedChoice` _aswbp_choice_scroller)))
        (:`CastFailed`
          _)))
    (:`else`
      _))
  (return 0))

(fn `GetOptionValueAsString`
  (returns (Value :type String))
  (bind _createdwidget (`self.CreatedWidget`)
    (:`then`
      (bind _aswbp_choice_scroller (cast `/Game/GenericShooter/Addons/MainMenu/Core/Controls/WBP_ChoiceScroller` _createdwidget)
        (:`then`
          (return (`/Game/GenericShooter/Addons/MainMenu/Core/Controls/WBP_ChoiceScroller.GetSelectedChoiceTag` _aswbp_choice_scroller)))
        (:`CastFailed`
          _)))
    (:`else`
      _))
  (return ""))

(fn `GetOptionValueAsURLString`
  (returns (URLString :type String))
  (bind _value (`self.GetOptionValueAsString`))
  (return (`KismetStringLibrary.Concat_StrStr` (`KismetStringLibrary.Conv_NameToString` (`self.OptionID`)) "=" _value)))