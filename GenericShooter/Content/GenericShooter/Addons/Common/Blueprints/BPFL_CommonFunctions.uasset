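; Blueprint function library of shared helpers for the GenericShooter addons, handling hit direction flags.
; MakeHitDirectionBitMask packs Left, Right, Top and Bottom booleans into a single integer bitmask, one bit per direction.
; GetHitDirectionBitFlags reverses this, using bitwise AND to unpack the mask into the four booleans.
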(fn `GetHitDirectionBitFlags`
  (params (HitDirectionBitMask :type Integer))
  (returns (bLeft :type Boolean) (bRight :type Boolean) (bTop :type Boolean) (bBottom :type Boolean))
  (return (`KismetMathLibrary.Conv_IntToBool` (`KismetMathLibrary.And_IntInt` HitDirectionBitMask 1)) (`KismetMathLibrary.Conv_IntToBool` (`KismetMathLibrary.And_IntInt` HitDirectionBitMask 2)) (`KismetMathLibrary.Conv_IntToBool` (`KismetMathLibrary.And_IntInt` HitDirectionBitMask 4)) (`KismetMathLibrary.Conv_IntToBool` (`KismetMathLibrary.And_IntInt` HitDirectionBitMask 8))))

(fn `MakeHitDirectionBitMask`
  (params (bLeft :type Boolean) (bRight :type Boolean) (bTop :type Boolean) (bBottom :type Boolean))
  (returns (HitDirectionBitMask :type Integer))
  (return (`KismetMathLibrary.Or_IntInt` (`KismetMathLibrary.Conv_BoolToInt` bLeft) (* (`KismetMathLibrary.Conv_BoolToInt` bRight) 2) (* (`KismetMathLibrary.Conv_BoolToInt` bTop) 4) (* (`KismetMathLibrary.Conv_BoolToInt` bBottom) 8))))