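; Base class for slot inventory item info, providing overridable hooks for spawning, syncing from actors, adding, invoking and bar fill display.
; SpawnActor and UpdateFromActor are stubs that print red on-screen errors when not implemented; the other hooks return simple defaults.
; An InitialSpawn flag gates one-time updates from an actor, including a temporary one spawned, read and destroyed.
; IsHigherPriorityThan ranks items by Slot and Priority.
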(fn `CanBeAdded`
  (params (InventoryOwner :type "Actor Object Reference") (ExistingItems :type "Array of /Game/GenericShooter/Addons/Common/Blueprints/BaseClasses/BP_SlotInventory_ItemInfo_Base Object Reference"))
  (returns (bCanBeAdded :type Boolean))
  (return true))

(fn `GetItemBarFillPercent`
  (returns (Percent :type "Float (double-precision)"))
  (return 0.5))

(fn `Invoke`
  (params (Invoker :type "Actor Object Reference"))
  (returns (bInvoked :type Boolean) (bShouldBeConsumed :type Boolean))
  (return false false))

(fn `IsHigherPriorityThan`
  (params (ItemInfo :type "/Game/GenericShooter/Addons/Common/Blueprints/BaseClasses/BP_SlotInventory_ItemInfo_Base Object Reference"))
  (returns (bHigher :type Boolean))
  (`/Engine/EditorBlueprintResources/StandardMacros.IsValid` ItemInfo
    (:`Is Valid`
      (return (and (<= (`self.Slot`) (`/Game/GenericShooter/Addons/Common/Blueprints/BaseClasses/BP_SlotInventory_ItemInfo_Base.Slot` ItemInfo)) (> (`self.Priority`) (`/Game/GenericShooter/Addons/Common/Blueprints/BaseClasses/BP_SlotInventory_ItemInfo_Base.Priority` ItemInfo)))))
    (:`Is Not Valid`
      (return true))))

(fn `SpawnActor`
  (params (OwningActor :type "Actor Object Reference") (Instigator :type "Pawn Object Reference") (bIsSpawningTempActor :type Boolean))
  (returns (NewActor :type "Actor Object Reference"))
  (`KismetSystemLibrary.PrintString` (`KismetTextLibrary.Conv_TextToString` (`|FormatText` "ERROR: Item Info Class '{ItemInfo}' tried to SpawnActor but does not have SpawnActor implemented!" (`KismetTextLibrary.Conv_StringToText` (`KismetSystemLibrary.GetDisplayName` self)))) true true (struct :`R` 1.0 :`G` 0.015037 :`A` 1.0) 10.0)
  (`self.UpdateFromActorIfInitialSpawn` null)
  (return null))

(fn `UpdateFromActor`
  (params (Actor :type "Actor Object Reference"))
  (returns (bUpdated :type Boolean))
  (`KismetSystemLibrary.PrintString` (`KismetTextLibrary.Conv_TextToString` (`|FormatText` "ERROR: Item Info Class '{ItemInfo}' tried to UpdateFromActor but does not have Update From Actor implemented!" (`KismetTextLibrary.Conv_StringToText` (`KismetSystemLibrary.GetDisplayName` self)))) true true (struct :`R` 1.0 :`G` 0.015037 :`A` 1.0) 10.0)
  (set `self.bInitialSpawn` false)
  (return false))

(fn `UpdateFromActorIfInitialSpawn`
  (params (Actor :type "Actor Object Reference"))
  (returns (bUpdated :type Boolean))
  (if (`self.bInitialSpawn`)
    (set `self.bInitialSpawn` false)
    (bind _bupdated (`self.UpdateFromActor` Actor))
    (return _bupdated)
    (else
      (return false))))

(fn `UpdateFromActorIfInitialSpawnUsingTempActor`
  (returns (bUpdated :type Boolean))
  (if (`self.bInitialSpawn`)
    (set `self.bInitialSpawn` false)
    (bind _newactor (`self.SpawnActor` null null true))
    (bind _bupdated (`self.UpdateFromActor` _newactor))
    (`self.K2_DestroyActor` _newactor)
    (return _bupdated)
    (else
      (return false))))

(fn `UserConstructionScript`)