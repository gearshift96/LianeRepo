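; Anim notify named "Footstep" that plays surface-appropriate footstep effects during character animations.
; If the owner has a CharacterMovementComponent, it skips the effect unless walking and scales volume by speed relative to a percentage of max walk speed.
; It then runs a short vertical line trace at the foot socket and passes the hit, effect category and volume to a physical-material effect spawner driven by a data table.
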(fn `GetNotifyName`
  (returns (ReturnValue :type String))
  (return "Footstep"))

(fn `Received_Notify`
  (params (MeshComp :type "SkeletalMeshComponent Object Reference") (Animation :type "AnimSequenceBase Object Reference"))
  (returns (ReturnValue :type Boolean))
  (locals (SocketLocation :type "Vector Structure") (VolumeScale :type "Float (double-precision)" :default 1.0) (OwningActor :type "Actor Object Reference") (CharacterMovementComponent :type "CharacterMovementComponent Object Reference"))
  (bind _returnvalue (`Actor.GetComponentByClass` (`local.OwningActor`) "/Script/Engine.CharacterMovementComponent"))
  (set `local.OwningActor` (`ActorComponent.GetOwner` MeshComp))
  (`|ExecutionSequence`
    (:`then_0`
      ;[1 1 1] Get character movement specific info if available, i.e. do nothing if we aren't walking, scale volume by speed...
      (set `local.CharacterMovementComponent` _returnvalue)
      (`/Engine/EditorBlueprintResources/StandardMacros.IsValid` _returnvalue
        (:`Is Valid`
          (if (`CharacterMovementComponent.IsWalking` _returnvalue)
            (set `local.VolumeScale` (`KismetMathLibrary.FClamp` (/ (`KismetMathLibrary.VSize` (`Actor.GetVelocity` (`local.OwningActor`))) (* (`CharacterMovementComponent.MaxWalkSpeed` (`local.CharacterMovementComponent`)) (`self.PercentageOfMaxWalkSpeedForFullVolume`)))))
            (else
              (return true))))))
    (:`then_1`
      ;[1 1 1] Grab what we are walking on and play an appropriate effect
      (bind _output_get (set `local.SocketLocation` (`SceneComponent.GetSocketLocation` (`local.MeshComp`) (`self.FootSocketName`))))
      (bind _outhit (`KismetSystemLibrary.LineTraceSingle` (+ _output_get (0.0 0.0 10.0)) (- _output_get (0.0 0.0 20.0)) "TraceTypeQuery1" false (`|MakeArray` (`local.OwningActor`))))
      (`/Game/GenericShooter/Addons/Common/Blueprints/BPFL_ImpactEffectFunctions.SpawnPhysicalMaterialEffectFromDataTable` (`self.EffectCategoryName`) (`self.FootstepEffectTable`) _outhit (`local.OwningActor`) (`local.VolumeScale`))
      (return true))))