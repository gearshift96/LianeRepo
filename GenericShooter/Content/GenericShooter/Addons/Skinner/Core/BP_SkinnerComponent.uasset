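; Actor component that skins its owner's tag-found first and third person meshes from a character DataTable row.
; Applying a row sets meshes, anim classes and dynamic materials, then reapplies stored scalar and vector overrides.
; Clients request skin changes by server RPC; RepNotifies reapply skins and parameters, skipping mismatched name/value arrays from partial updates.
; The chosen key can persist in a prefixed save slot and optionally load on BeginPlay.
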(event `ServerSetCharacterKeyName`
  (params (CharacterKeyName :type Name))
  ;[1 1 1] Tell Server we want to change our character key name
  (if (and (== CharacterKeyName (`self.CharacterKeyName`)) (not (`.bIsLocallyControlled` (`self.GetLocalUserIndexIfExists`))))
    (`|ExecutionSequence`
      (:`then_0`
        (set `self.CharacterKeyName` CharacterKeyName :!label _label)
        (`self.PrintDebugString` (`KismetStringLibrary.Concat_StrStr` "Server Set Character Name To: " (`KismetStringLibrary.Conv_NameToString` CharacterKeyName)))
        (`self.ApplyToOwner`))
      (:`then_1`
        (`self.ForceClientToReApply`)))
    (else
      (goto _label))))

(event `ForceClientToReApply`
  (`self.ApplyToOwnerIfClientOnly`))

(event `self.ReceiveBeginPlay`
  (`KismetSystemLibrary.Delay` 0.0)
  (`self.PerformSpawnBehavior`))

(fn `ApplyMaterialParameterOverrides`
  (`self.PrintDebugString` "Applying ALL material parameter overrides.")
  (`|ExecutionSequence`
    (:`then_0`
      ;[1 1 1] Make sure scalar data is valid before trying to apply. We might be invalid if we get a partial update because networking is hard.
      (if (== (`KismetArrayLibrary.Array_Length` (`self.ScalarValues`)) (`KismetArrayLibrary.Array_Length` (`self.ScalarParameters`)))
        ;[1 1 1] Loop through scalars and apply them
        (for (_array_element _array_index) (`self.ScalarParameters`)
          (bind _skeletalmeshcomponents (`self.GetValidMeshComponents`))
          (`MeshComponent.SetScalarParameterValueOnMaterials` _skeletalmeshcomponents _array_element (`|GetArrayItem` (`self.ScalarValues`) _array_index)))))
    (:`then_1`
      ;[1 1 1] Make sure vector data is valid before trying to apply. We might be invalid if we get a partial update because networking is hard.
      (if (== (`KismetArrayLibrary.Array_Length` (`self.VectorParameters`)) (`KismetArrayLibrary.Array_Length` (`self.VectorValues`)))
        ;[1 1 1] Loop through vectors and apply them
        (for (_array_element_2 _array_index_2) (`self.VectorParameters`)
          (bind _skeletalmeshcomponents_2 (`self.GetValidMeshComponents`))
          (`MeshComponent.SetVectorParameterValueOnMaterials` _skeletalmeshcomponents_2 _array_element_2 (`|GetArrayItem` (`self.VectorValues`) _array_index_2)))))
    (:`then_2`
      (return))))

(fn `ApplyToOwner`
  (locals (ThirdPersonMesh :type "SkeletalMesh Object Reference") (MaterialIndex :type Integer) (FirstPersonMesh :type "SkeletalMesh Object Reference"))
  (bind _materialindex (`local.MaterialIndex`))
  (bind _materialindex_2 (`local.MaterialIndex`))
  (bind _materialindex_3 (`local.MaterialIndex`))
  (bind _materialindex_4 (`local.MaterialIndex`))
  (`self.PrintDebugString` "Applying skin to owner.")
  ;[1 1 1] Make sure Data table is valid
  (`/Engine/EditorBlueprintResources/StandardMacros.IsValid` (`self.CharacterDataTable`)
    (:`Is Valid`
      ;[1 1 1] If both components are null, attempt to get mesh components
      (if (`KismetMathLibrary.BooleanNOR` (`KismetSystemLibrary.IsValid` (`self.ThirdPersonMeshComponent`)) (`KismetSystemLibrary.IsValid` (`self.FirstPersonMeshComponent`)))
        (`self.GetMeshComponents`))
      ;[1 1 1] If we don't find character info data, simply bail
      (bind _returnvalue (`|GetDataTableRow` (`self.CharacterDataTable`) (`self.CharacterKeyName`))
        (:`then`
          ;[1 1 1] Apply meshes, thirdperson anim instances, and materials
          (`|ExecutionSequence`
            (:`then_0`
              (bind (_userfriendlyname _animsetname _thirdpersonmesh _thirdpersonanimbp _thirdpersonmeshmaterialoverrides _firstpersonmesh _firstpersonanimbp _firstpersonmeshmaterialoverrides) (break `/Game/GenericShooter/Addons/Skinner/Core/FCharacterMeshInfo` _returnvalue))
              (set `local.ThirdPersonMesh` _thirdpersonmesh)
              (bind _thirdpersonmeshcomponent (`self.ThirdPersonMeshComponent`)
                (:`then`
                  (`SkinnedMeshComponent.SetSkinnedAssetAndUpdate` _thirdpersonmeshcomponent (`local.ThirdPersonMesh`) false)
                  (`SkeletalMeshComponent.K2_SetAnimInstanceClass` _thirdpersonmeshcomponent _thirdpersonanimbp)
                  (for _index (range (`PrimitiveComponent.GetNumMaterials` (`self.ThirdPersonMeshComponent`)))
                    (set `local.MaterialIndex` _index)
                    (if (`KismetArrayLibrary.Array_IsValidIndex` _thirdpersonmeshmaterialoverrides _materialindex_2)
                      (`PrimitiveComponent.CreateDynamicMaterialInstance` (`self.ThirdPersonMeshComponent`) _materialindex (`|GetArrayItem` _thirdpersonmeshmaterialoverrides _materialindex_2) "None")
                      (else
                        (`PrimitiveComponent.CreateDynamicMaterialInstance` (`self.ThirdPersonMeshComponent`) _materialindex (`.MaterialInterface` (break `SkeletalMaterial` (`|GetArrayItem` (`SkeletalMesh.Materials` (`local.ThirdPersonMesh`)) (`local.MaterialIndex`)))) "None") ; Create a mid from the original mesh material if no override present
                      ))))
                (:`else`)))
            (:`then_1`
              (set `local.FirstPersonMesh` _firstpersonmesh)
              (bind _firstpersonmeshcomponent (`self.FirstPersonMeshComponent`)
                (:`then`
                  (`SkinnedMeshComponent.SetSkinnedAssetAndUpdate` _firstpersonmeshcomponent (`local.FirstPersonMesh`) false)
                  (`SkeletalMeshComponent.K2_SetAnimInstanceClass` _firstpersonmeshcomponent _firstpersonanimbp)
                  (for _index_2 (range (`PrimitiveComponent.GetNumMaterials` (`self.FirstPersonMeshComponent`)))
                    (set `local.MaterialIndex` _index_2)
                    (if (`KismetArrayLibrary.Array_IsValidIndex` _firstpersonmeshmaterialoverrides _materialindex_4)
                      (`PrimitiveComponent.CreateDynamicMaterialInstance` (`self.FirstPersonMeshComponent`) _materialindex_3 (`|GetArrayItem` _firstpersonmeshmaterialoverrides _materialindex_4) "None")
                      (else
                        (`PrimitiveComponent.CreateDynamicMaterialInstance` (`self.FirstPersonMeshComponent`) _materialindex_3 (`.MaterialInterface` (break `SkeletalMaterial` (`|GetArrayItem` (`SkeletalMesh.Materials` (`local.FirstPersonMesh`)) _index_2))) "None") ; Create a mid from the original mesh material if no override present
                      ))))
                (:`else`)))
            (:`then_2`
              (`self.ApplyMaterialParameterOverrides`)
              (set `self.CharacterAnimSetName` _animsetname)
              (`self.OnSkinApplied` (`self.CharacterKeyName`))
              (return))))
        (:`RowNotFound`
          (`self.PrintDebugString` "Could not find character info in data table.")
          (return))))
    (:`Is Not Valid`
      (`self.PrintDebugString` "Character data table invalid.")
      (return))))

(fn `ApplyToOwnerIfClientOnly`
  (`self.PrintDebugString` "Applying to owner if client only")
  (if (not (`KismetSystemLibrary.IsServer`))
    (`self.ApplyToOwner`)
    (return)
    (else
      (return))))

(fn `ChangeCharacterSkin`
  (params (NewCharacterKeyName :type Name) (bSave :type Boolean) (bSaveIfLocal :type Boolean))
  ;[1 1 1] Emit debug info if debug enabled
  (`self.PrintDebugString` (`KismetStringLibrary.Concat_StrStr` "Changing Character Skin To: " (`KismetStringLibrary.Conv_NameToString` NewCharacterKeyName)))
  ;[1 1 1] If we're in a multiplayer game and are not the server, tell the server to set our character name, otherwise...
  (if (and (not (`KismetSystemLibrary.IsServer`)) (not (`KismetSystemLibrary.IsStandalone`)))
    (`self.ServerSetCharacterKeyName` (`local.NewCharacterKeyName`))
    (return)
    (else
      ;[1 1 1] ...set character name and apply it to our owner. If we are to save, handle save logic.
      (set `self.CharacterKeyName` (`local.NewCharacterKeyName`))
      (`self.ApplyToOwner`)
      (if (`local.bSave`)
        (if (`local.bSaveIfLocal`)
          (`self.SaveKeyNameIfLocal`)
          (return)
          (else
            (`self.SaveKeyName` 0)
            (return)))
        (else
          (return))))))

(fn `ClearAllMaterialParameterOverrides`
  (`KismetArrayLibrary.Array_Clear` (`self.ScalarParameters`))
  (`KismetArrayLibrary.Array_Clear` (`self.VectorParameters`))
  (`KismetArrayLibrary.Array_Clear` (`self.ScalarValues`))
  (`KismetArrayLibrary.Array_Clear` (`self.VectorValues`))
  (return))

(fn `GetLocalUserIndexIfExists`
  (returns (ID :type Integer) (bIsLocallyControlled :type Boolean))
  ;[1 1 1] If owner is not a pawn, we can't get the local user
  (bind _aspawn (cast `Pawn` (`self.GetOwner`))
    (:`then`
      ;[1 1 1] If not locally controlled, we can't get the local user id
      (if (`Pawn.IsLocallyControlled` _aspawn)
        ;[1 1 1] Are locally controlled, so get our user id
        (bind _returnvalue (`GameplayStatics.GetPlayerControllerID` (cast `PlayerController` (`Pawn.GetController` _aspawn) :!pure true)))
        (return _returnvalue true)
        (else
          (return 0 false))))
    (:`CastFailed`
      (return 0 false))))

(fn `GetMaterialScalarParameter`
  (params (ScalarParameterName :type Name))
  (returns (Value :type "Float (double-precision)") (bFound :type Boolean))
  (locals (Index :type Integer))
  (bind _output_get (set `local.Index` (`KismetArrayLibrary.Array_Find` (`self.ScalarParameters`) ScalarParameterName)))
  (if (!= _output_get -1)
    (return (`|GetArrayItem` (`self.ScalarValues`) (`local.Index`)) true)
    (else
      (return 0.0 false))))

(fn `GetMaterialVectorParameter`
  (params (VectorParameterName :type Name))
  (returns (Value :type "Vector Structure") (bFound :type Boolean))
  (locals (Index :type Integer))
  (bind _output_get (set `local.Index` (`KismetArrayLibrary.Array_Find` (`self.VectorParameters`) VectorParameterName)))
  (if (!= _output_get -1)
    (return (`|GetArrayItem` (`self.VectorValues`) (`local.Index`)) true)
    (else
      (return (0.0 0.0 0.0) false))))

(fn `GetMeshComponents`
  (bind _returnvalue (`Actor.GetComponentsByTag` (`self.GetOwner`) "/Script/Engine.SkeletalMeshComponent" (`self.FirstPersonMeshComponentTag`)))
  (bind _returnvalue_2 (`Actor.GetComponentsByTag` (`self.GetOwner`) "/Script/Engine.SkeletalMeshComponent" (`self.ThirdPersonMeshComponentTag`)))
  ;[1 1 1] Make sure we have an owner and its not being destroyed
  (`/Engine/EditorBlueprintResources/StandardMacros.IsValid` (`self.GetOwner`)
    (:`Is Valid`
      (`|ExecutionSequence`
        (:`then_0`
          ;[1 1 1] Get Third Person Mesh Component
          (if (`KismetArrayLibrary.Array_IsValidIndex` _returnvalue_2)
            (set `self.ThirdPersonMeshComponent` (`|GetArrayItem` _returnvalue_2))))
        (:`then_1`
          ;[1 1 1] Get First Person Mesh Component
          (if (`KismetArrayLibrary.Array_IsValidIndex` _returnvalue)
            (set `self.FirstPersonMeshComponent` (`|GetArrayItem` _returnvalue))))
        (:`then_2`
          (return))))
    (:`Is Not Valid`
      (return))))

(fn `GetValidMeshComponents`
  (returns (SkeletalMeshComponents :type "Array of SkeletalMeshComponent Object Reference"))
  (locals (OutMeshComponents :type "Array of SkeletalMeshComponent Object Reference"))
  ;[1 1 1] Outputs our valid skeletal meshes
  (bind _thirdpersonmeshcomponent (`self.ThirdPersonMeshComponent`)
    (:`then`
      (`KismetArrayLibrary.Array_Add` (`local.OutMeshComponents`) _thirdpersonmeshcomponent))
    (:`else`
      _))
  (bind _firstpersonmeshcomponent (`self.FirstPersonMeshComponent`)
    (:`then`
      (`KismetArrayLibrary.Array_Add` (`local.OutMeshComponents`) _firstpersonmeshcomponent))
    (:`else`
      _))
  (return (`local.OutMeshComponents`)))

(fn `LoadKeyName`
  (params (UserIndex :type Integer))
  (returns (CharacterKeyName :type Name) (bLoaded :type Boolean))
  (locals (SaveName :type String))
  ;[1 1 1] To allow multiple skin saves, we have a configurable prefix that components can use.
  (bind _output_get (set `local.SaveName` (`KismetStringLibrary.Concat_StrStr` (`KismetStringLibrary.Conv_NameToString` (`self.ReadFromSaveSlotPrefix`)) "_BasicSkinSave")))
  ;[1 1 1] If save data doesn't exist, simply return whatever our current character key name is
  (bind _returnvalue (`GameplayStatics.DoesSaveGameExist` _output_get (`local.UserIndex`)))
  (if _returnvalue
    ;[1 1 1] Load save game from slot and return loaded key. This cast shouldn't ever fail.
    (bind _returnvalue_2 (`GameplayStatics.LoadGameFromSlot` (`local.SaveName`) (`local.UserIndex`)))
    (bind _asbp_skinner_save_data (cast `/Game/GenericShooter/Addons/Skinner/Core/BP_SkinnerSaveData` _returnvalue_2)
      (:`then`
        (return (`/Game/GenericShooter/Addons/Skinner/Core/BP_SkinnerSaveData.CharacterKeyName` _asbp_skinner_save_data) true))
      (:`CastFailed`
        (`self.PrintDebugString` "Failed to load skin save data.")
        (return (`self.CharacterKeyName`) false)))
    (else
      (`self.PrintDebugString` "Skin save data doesn't exist.")
      (return (`self.CharacterKeyName`) false))))

(fn `OnRep_CharacterDataTable`
  (`self.ApplyToOwnerIfClientOnly`)
  (return))

(fn `OnRep_CharacterKeyName`
  (`self.ApplyToOwnerIfClientOnly`)
  (return))

(fn `OnRep_ScalarParameters`
  (`self.ApplyMaterialParameterOverrides`)
  (return))

(fn `OnRep_ScalarValues`
  (`self.ApplyMaterialParameterOverrides`)
  (return))

(fn `OnRep_VectorParameters`
  (`self.ApplyMaterialParameterOverrides`)
  (return))

(fn `OnRep_VectorValues`
  (`self.ApplyMaterialParameterOverrides`)
  (return))

(fn `PerformSpawnBehavior`
  (locals (bApplied :type Boolean))
  (bind (_characterkeyname _bloaded) (`self.LoadKeyName` 0))
  (bind (_id _bislocallycontrolled) (`self.GetLocalUserIndexIfExists`))
  (`self.PrintDebugString` "Performing Spawn Behavior")
  (`|ExecutionSequence`
    (:`then_0`
      ;[1 1 1] If force load enabled, go ahead and load without doing a local id check (currently means we have to load from user 0)
      (if (and (`self.bForceLoadAndNotify`) _bloaded)
        (`self.ChangeCharacterSkin` _characterkeyname)
        (set `local.bApplied` true)
        (else
          ;[1 1 1] If loading if local only, do that now if we're local
          (if (`self.bLoadLocalAndNotifyServerOnBeginPlay`)
            (if _bislocallycontrolled
              (`self.ChangeCharacterSkin` (`self.LoadKeyName` _id))
              (set `local.bApplied` true)
              (else
                (`self.PrintDebugString` "Failed to load local and notify server.")))
            (else
              (`self.PrintDebugString` "Did no loading."))))))
    (:`then_1`
      ;[1 1 1] Apply if Apply On Begin Play is set and we haven't already applied ourselves through loading
      (if (and (`self.bApplyOnBeginPlay`) (not (`local.bApplied`)))
        (`self.ApplyToOwner`)
        (return)
        (else
          (return))))))

(fn `SaveKeyName`
  (params (UserIndex :type Integer))
  (returns (bSaved :type Boolean))
  (locals (SlotName :type String) (SaveData :type "/Game/GenericShooter/Addons/Skinner/Core/BP_SkinnerSaveData Object Reference"))
  ;[1 1 1] To allow multiple skin saves, we have a configurable prefix that components can use.
  (set `local.SlotName` (`KismetStringLibrary.Concat_StrStr` (`KismetStringLibrary.Conv_NameToString` (`self.ReadFromSaveSlotPrefix`)) "_BasicSkinSave"))
  ;[1 1 1] If we can't load save data, we'll just make a new save game object
  (bind _returnvalue (`GameplayStatics.LoadGameFromSlot` (`local.SlotName`) (`local.UserIndex`)))
  (bind _asbp_skinner_save_data (cast `/Game/GenericShooter/Addons/Skinner/Core/BP_SkinnerSaveData` _returnvalue)
    (:`then`
      (set `local.SaveData` _asbp_skinner_save_data))
    (:`CastFailed`
      (bind _returnvalue_2 (`GameplayStatics.CreateSaveGameObject` "/Game/GenericShooter/Addons/Skinner/Core/BP_SkinnerSaveData.BP_SkinnerSaveData_C"))
      (set `local.SaveData` _returnvalue_2)))
  ;[1 1 1] Set save data, then save it
  (set `/Game/GenericShooter/Addons/Skinner/Core/BP_SkinnerSaveData.CharacterKeyName` (`self.CharacterKeyName`) (`local.SaveData`))
  (bind _returnvalue_3 (`GameplayStatics.SaveGameToSlot` (`local.SaveData`) (`local.SlotName`) (`local.UserIndex`)))
  (return _returnvalue_3))

(fn `SaveKeyNameIfLocal`
  (bind (_id _bislocallycontrolled) (`self.GetLocalUserIndexIfExists`))
  ;[1 1 1] Only saves if we can guarantee the owner is a locally controlled character
  (if _bislocallycontrolled
    (`self.SaveKeyName` _id)
    (return)
    (else
      (return))))

(fn `SetMaterialScalarParameter`
  (params (ParameterName :type Name) (Scalar :type "Float (double-precision)") (bRelative :type Boolean))
  (locals (NewScalarValue :type "Float (double-precision)") (ParameterIndex :type Integer))
  (`|ExecutionSequence`
    (:`then_0`
      ;[1 1 1] If relative, get current value and add to it
      (if (`local.bRelative`)
        (set `local.NewScalarValue` (+ (`local.Scalar`) (`self.GetMaterialScalarParameter` (`local.ParameterName`))))
        (else
          (set `local.NewScalarValue` (`local.Scalar`)))))
    (:`then_1`
      ;[1 1 1] Add or update scalar parameter info
      (bind _output_get (set `local.ParameterIndex` (`KismetArrayLibrary.Array_Find` (`self.ScalarParameters`) (`local.ParameterName`))))
      (if (== _output_get -1)
        (`KismetArrayLibrary.Array_Add` (`self.ScalarParameters`) (`local.ParameterName`))
        (`KismetArrayLibrary.Array_Add` (`self.ScalarValues`) (`local.NewScalarValue`))
        (else
          (`KismetArrayLibrary.Array_Set` (`self.ScalarValues`) (`local.ParameterIndex`) (`local.NewScalarValue`)))))
    (:`then_2`
      ;[1 1 1] Apply the new scalar parameter value to materials
      (`self.PrintDebugString` (`KismetStringLibrary.Concat_StrStr` "Setting a scalar parameter material value: " (`KismetStringLibrary.Conv_NameToString` (`local.ParameterName`))))
      (bind _skeletalmeshcomponents (`self.GetValidMeshComponents`))
      (`MeshComponent.SetScalarParameterValueOnMaterials` _skeletalmeshcomponents (`local.ParameterName`) (`local.NewScalarValue`)) ; Apply the new parameter
      (return))))

(fn `SetMaterialVectorParameter`
  (params (ParameterName :type Name) (Vector :type "Vector Structure"))
  (locals (ParameterIndex :type Integer))
  (`|ExecutionSequence`
    (:`then_0`
      ;[1 1 1] Add or update vector parameter info
      (bind _output_get (set `local.ParameterIndex` (`KismetArrayLibrary.Array_Find` (`self.VectorParameters`) (`local.ParameterName`))))
      (if (== _output_get -1)
        (`KismetArrayLibrary.Array_Add` (`self.VectorParameters`) (`local.ParameterName`))
        (`KismetArrayLibrary.Array_Add` (`self.VectorValues`) (`local.Vector`))
        (else
          (`KismetArrayLibrary.Array_Set` (`self.VectorValues`) (`local.ParameterIndex`) (`local.Vector`)))))
    (:`then_1`
      ;[1 1 1] Apply new vector parameter info
      (`self.PrintDebugString` (`KismetStringLibrary.Concat_StrStr` "Setting a vector parameter material value: " (`KismetStringLibrary.Conv_NameToString` (`local.ParameterName`))))
      (bind _skeletalmeshcomponents (`self.GetValidMeshComponents`))
      (`MeshComponent.SetVectorParameterValueOnMaterials` _skeletalmeshcomponents (`local.ParameterName`) (`local.Vector`))
      (return))))