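; Replication helper actor for the StatManager addon that exposes stat reading and writing through a single actor.
; Each function forwards directly to a BPStatManager reference and returns its result, holding no logic of its own.
; The wrapped API covers getting, setting and incrementing float and int stats, getting and setting string stats, listing stored stats, and checking whether a client may set a stat.
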(fn `CanClientSetStat`
  (params (StatName :type Name))
  (returns (bCanSet :type Boolean))
  (bind _bcanset (`/Game/GenericShooter/Addons/StatManager/Core/BP_StatManagerComponent.CanClientSetStat` (`self.BP_StatManager`) StatName))
  (return _bcanset))

(fn `GetAllStoredFloatStats`
  (returns (OutFloatStatNames :type "Array of Name") (OutFloatStatValues :type "Array of Float (double-precision)"))
  (bind (_outfloatstatnames _outfloatstatvalues) (`/Game/GenericShooter/Addons/StatManager/Core/BP_StatManagerComponent.GetAllStoredFloatStats` (`self.BP_StatManager`)))
  (return _outfloatstatnames _outfloatstatvalues))

(fn `GetAllStoredIntStats`
  (returns (OutIntStatNames :type "Array of Name") (OutIntStatValues :type "Array of Integer"))
  (bind (_outintstatnames _outintstatvalues) (`/Game/GenericShooter/Addons/StatManager/Core/BP_StatManagerComponent.GetAllStoredIntStats` (`self.BP_StatManager`)))
  (return _outintstatnames _outintstatvalues))

(fn `GetAllStoredStringStats`
  (returns (OutStringStatNames :type "Array of Name") (OutStringStatValues :type "Array of String"))
  (bind (_outstringstatnames _outstringstatvalues) (`/Game/GenericShooter/Addons/StatManager/Core/BP_StatManagerComponent.GetAllStoredStringStats` (`self.BP_StatManager`)))
  (return _outstringstatnames _outstringstatvalues))

(fn `GetFloatStat`
  (params (StatName :type Name) (DefaultValue :type "Float (double-precision)"))
  (returns (StatValue :type "Float (double-precision)"))
  (bind _statvalue (`/Game/GenericShooter/Addons/StatManager/Core/BP_StatManagerComponent.GetFloatStat` (`self.BP_StatManager`) StatName DefaultValue))
  (return _statvalue))

(fn `GetIntStat`
  (params (StatName :type Name) (DefaultValue :type Integer))
  (returns (StatValue :type Integer))
  (bind _statvalue (`/Game/GenericShooter/Addons/StatManager/Core/BP_StatManagerComponent.GetIntStat` (`self.BP_StatManager`) StatName DefaultValue))
  (return _statvalue))

(fn `GetStringStat`
  (params (StatName :type Name) (DefaultValue :type String))
  (returns (StatValue :type String))
  (bind _statvalue (`/Game/GenericShooter/Addons/StatManager/Core/BP_StatManagerComponent.GetStringStat` (`self.BP_StatManager`) StatName DefaultValue))
  (return _statvalue))

(fn `IncrementFloatStat`
  (params (StatName :type Name) (Amount :type "Float (double-precision)"))
  (returns (NewValue :type "Float (double-precision)"))
  (bind _newvalue (`/Game/GenericShooter/Addons/StatManager/Core/BP_StatManagerComponent.IncrementFloatStat` (`self.BP_StatManager`) StatName Amount))
  (return _newvalue))

(fn `IncrementIntStat`
  (params (StatName :type Name) (Amount :type Integer))
  (returns (NewValue :type Integer))
  (bind _newvalue (`/Game/GenericShooter/Addons/StatManager/Core/BP_StatManagerComponent.IncrementIntStat` (`self.BP_StatManager`) StatName Amount))
  (return _newvalue))

(fn `SetFloatStat`
  (params (StatValue :type Name) (NewValue :type "Float (double-precision)"))
  (returns (bWasNewlyAdded :type Boolean))
  (bind _bwasnewlyadded (`/Game/GenericShooter/Addons/StatManager/Core/BP_StatManagerComponent.SetFloatStat` (`self.BP_StatManager`) StatValue NewValue))
  (return _bwasnewlyadded))

(fn `SetIntStat`
  (params (StatName :type Name) (NewValue :type Integer))
  (returns (bWasNewlyAdded :type Boolean))
  (bind _bwasnewlyadded (`/Game/GenericShooter/Addons/StatManager/Core/BP_StatManagerComponent.SetIntStat` (`self.BP_StatManager`) StatName NewValue))
  (return _bwasnewlyadded))

(fn `SetStringStat`
  (params (StatName :type Name) (StatValue :type String))
  (returns (bWasNewlyAdded :type Boolean))
  (bind _bwasnewlyadded (`/Game/GenericShooter/Addons/StatManager/Core/BP_StatManagerComponent.SetStringStat` (`self.BP_StatManager`) StatName StatValue))
  (return _bwasnewlyadded))

(fn `UserConstructionScript`)