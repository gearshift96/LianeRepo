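; BP_SettingsManagerHelper is a helper Blueprint for the Settings Manager addon that applies audio settings through sound mixes.
; SetBaseSoundMix passes a given mix through to the engine's base mix call.
; SetSoundMixVolumeOverride switches on a class name (Master, SFX, Music, UI or Announcer) to set that sound class's volume override on the supplied mix with no fade.
; Unhandled names print an error.
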(fn `SetBaseSoundMix`
  (params (SoundMix :type "SoundMix Object Reference"))
  (`GameplayStatics.SetBaseSoundMix` SoundMix)
  (return))

(fn `SetSoundMixVolumeOverride`
  (params (MasterMix :type "SoundMix Object Reference") (Volume :type "Float (double-precision)") (SoundClassName :type Name))
  (switch `name` SoundClassName
    (:`Default`
      (`KismetSystemLibrary.PrintString` "ERROR: SetSoundMixVolumeOverride did not handle SoundClassName correctly!" true true (struct :`R` 1.0 :`B` 0.012564 :`A` 1.0) 10.0)
      (return))
    (:`Master`
      (`GameplayStatics.SetSoundMixClassOverride` (`local.MasterMix`) "/Game/GenericShooter/Addons/Common/Audio/Master.Master" (`local.Volume`) 1.0 0.0))
    (:`SFX`
      (`GameplayStatics.SetSoundMixClassOverride` (`local.MasterMix`) "/Game/GenericShooter/Addons/Common/Audio/SFX.SFX" (`local.Volume`) 1.0 0.0))
    (:`Music`
      (`GameplayStatics.SetSoundMixClassOverride` (`local.MasterMix`) "/Game/GenericShooter/Addons/Common/Audio/Music.Music" (`local.Volume`) 1.0 0.0))
    (:`UI`
      (`GameplayStatics.SetSoundMixClassOverride` (`local.MasterMix`) "/Game/GenericShooter/Addons/Common/Audio/UI.UI" (`local.Volume`) 1.0 0.0))
    (:`Announcer`
      (`GameplayStatics.SetSoundMixClassOverride` (`local.MasterMix`) "/Game/GenericShooter/Addons/Common/Audio/Announcer.Announcer" (`local.Volume`) 1.0 0.0)))
  (return))

(fn `UserConstructionScript`)