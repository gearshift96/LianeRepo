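; Base SaveGame class for a settings bucket in the Settings Manager addon, holding settings that persist in their own save slot.
; InitializeDefaults and ApplySettings are stubs returning true, apparently meant for child buckets to override.
; SaveDefaults stores the slot prefix, initializes defaults and saves, while SaveCurrent re-saves under the same prefix plus BucketName slot.
; It also fetches a temporary settings helper from the SettingsManager, printing an error if invalid.
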(fn `ApplySettings`
  (returns (bApplied :type Boolean))
  (return true))

(fn `GetTemporarySettingsHelper`
  (returns (Helper :type "/Game/GenericShooter/Addons/SettingsManager/Core/BP_SettingsManagerHelper Object Reference"))
  (bind _settingsmanager (`self.SettingsManager`)
    (:`then`
      (bind _helper (`/Game/GenericShooter/Addons/SettingsManager/Core/BP_SettingsManager.GetTemporarySettingsManagerHelper` _settingsmanager))
      (return _helper))
    (:`else`
      (`KismetSystemLibrary.PrintString` null "ERROR: Settings Bucket can't get temporary settings helper because Settings Manager is invalid!" true true (struct :`R` 1.0 :`G` 0.015914 :`A` 1.0) 10.0)
      (return null))))

(fn `InitializeDefaults`
  (returns (bInitialized :type Boolean))
  (return true))

(fn `SaveCurrent`
  (returns (bSaved :type Boolean))
  (bind _returnvalue (`GameplayStatics.SaveGameToSlot` self (`KismetStringLibrary.Concat_StrStr` (`self.SlotNamePrefix`) (`KismetStringLibrary.Conv_NameToString` (`self.BucketName`)))))
  (return _returnvalue))

(fn `SaveDefaults`
  (params (SlotNamePrefix :type String))
  (bind _output_get (set `self.SlotNamePrefix` SlotNamePrefix))
  (`self.InitializeDefaults`)
  (`GameplayStatics.SaveGameToSlot` self (`KismetStringLibrary.Concat_StrStr` _output_get (`KismetStringLibrary.Conv_NameToString` (`self.BucketName`))))
  (return))