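; Base weapon actor for the shooter's weapon system, with overridable fire, ADS and throw hooks.
; Gathers fire mechanic components at construction and forwards their pre-fire, post-fire and animation requests through its own dispatchers.
; Server or standalone reloads move ammo from an interface-based reserve, restored on clients via RepNotify, into the loaded ammo storage component.
; Ammo changes broadcast vitals updates, and helpers expose ammo info, crosshair visibility, FOV and recoil spread.
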(event `self.BP_AmmoStorageComponent.OnAmmoChanged`
  (`self.OnVitalsChanged`))

(event `self.ReceiveBeginPlay`
  ;[1 1 1] Bind Pre and Post fire in our firing mechanics, as well as animation requests
  (for _array_element (`self.FiringMechanicComponents`)
    (add `/Game/GenericShooter/Addons/WeaponSystem/Core/BP_Weapon_FireMechanicBaseComponent.OnPreFire` _array_element (delegate `ForwardFiringMechanicPreFire`))
    (add `/Game/GenericShooter/Addons/WeaponSystem/Core/BP_Weapon_FireMechanicBaseComponent.OnPostFire` _array_element (delegate `ForwardFiringMechanicPostFire`))
    (add `/Game/GenericShooter/Addons/WeaponSystem/Core/BP_Weapon_FireMechanicBaseComponent.OnRequestPlayWeaponAnimation` _array_element (`|CreateDelegate` :!event `OnFireMechanicRequestedAnimation`))))

(event `ForwardFiringMechanicPreFire`
  (params (FiringMechanicComponent :type "/Game/GenericShooter/Addons/WeaponSystem/Core/BP_Weapon_FireMechanicBaseComponent Object Reference") (bSimulated :type Boolean))
  ;[1 1 1] Bind Pre and Post fire in our firing mechanics, as well as animation requests
  (`self.OnFiringMechanicPreFire` FiringMechanicComponent bSimulated))

(event `ForwardFiringMechanicPostFire`
  (params (FiringMechanicComponent :type "/Game/GenericShooter/Addons/WeaponSystem/Core/BP_Weapon_FireMechanicBaseComponent Object Reference") (bSimulated :type Boolean))
  ;[1 1 1] Bind Pre and Post fire in our firing mechanics, as well as animation requests
  (`self.OnFiringMechanicPostFire` FiringMechanicComponent bSimulated))

(fn `CanADS`
  (returns (bCanADS :type Boolean))
  (return true))

(fn `CanBeThrown`
  (returns (bCanBeThrown :type Boolean))
  (return true))

(fn `CanReload`
  (returns (bCanReload :type Boolean))
  (`/Engine/EditorBlueprintResources/StandardMacros.IsValid` (`KismetSystemLibrary.Conv_InterfaceToObject` (`self.ReserveAmmoStorage`))
    (:`Is Valid`
      ;[1 1 1] Does reserve ammo have ammo we need?
      (if (`/Game/GenericShooter/Addons/WeaponSystem/Core/BPFL_AmmoStorageFunctions.CanAmmoStoragePullAnyAmmoFromAnother` (`self.BP_AmmoStorageComponent`) (`self.ReserveAmmoStorage`))
        ;[1 1 1] Make sure firing mechanics can reload
        (for _array_element (`self.FiringMechanicComponents`)
          (if (not (`/Game/GenericShooter/Addons/WeaponSystem/Core/BP_Weapon_FireMechanicBaseComponent.CanReload` _array_element))
            (return false)))
        (return true)
        (else
          (return false))))
    (:`Is Not Valid`
      (return false))))

(fn `GetCrosshairVisibility`
  (returns (bShowCrosshair :type Boolean))
  (bind _returnvalue (`self.GetOwner`))
  (`/Engine/EditorBlueprintResources/StandardMacros.IsValid` _returnvalue
    (:`Is Valid`
      (bind _bvisibile (message `/Game/GenericShooter/Addons/Common/Blueprints/Interfaces/BPI_WeaponSystem_Holder.GetWeaponCrosshairVisibility` _returnvalue))
      (return _bvisibile))
    (:`Is Not Valid`
      (return false))))

(fn `GetDesiredFieldOfView`
  (params (ADSPosition :type "Float (double-precision)"))
  (returns (FOV :type "Float (double-precision)"))
  (return (`KismetMathLibrary.Lerp` (`self.BaseFOV`) (`self.ADSFOV`) (`KismetMathLibrary.FClamp` ADSPosition))))

(fn `GetLoadedAmmoInfoForAmmoType`
  (params (AmmoType :type "/Game/GenericShooter/Addons/WeaponSystem/Core/EWeaponAmmoType Enum" :default "NewEnumerator3"))
  (returns (AmmoInfo :type "/Game/GenericShooter/Addons/WeaponSystem/Core/FWeaponAmmoStorage Structure"))
  (bind _ammoinfo (`/Game/GenericShooter/Addons/WeaponSystem/Core/BP_AmmoStorageComponent.GetAmmoInfoForAmmoType` (`self.BP_AmmoStorageComponent`) AmmoType))
  (return _ammoinfo))

(fn `GetLoadedAmmoStorageCopy`
  (returns (AmmoStorage :type "Array of /Game/GenericShooter/Addons/WeaponSystem/Core/FWeaponAmmoStorage Structure"))
  (return (`/Game/GenericShooter/Addons/WeaponSystem/Core/BP_AmmoStorageComponent.AmmoStorage` (`self.BP_AmmoStorageComponent`))))

(fn `GetReserveAmmoInfoForAmmoType`
  (params (AmmoType :type "/Game/GenericShooter/Addons/WeaponSystem/Core/EWeaponAmmoType Enum" :default "NewEnumerator3"))
  (returns (AmmoInfo :type "/Game/GenericShooter/Addons/WeaponSystem/Core/FWeaponAmmoStorage Structure"))
  (bind _reserveammostorage (`self.ReserveAmmoStorage`))
  (`/Engine/EditorBlueprintResources/StandardMacros.IsValid` (`KismetSystemLibrary.Conv_InterfaceToObject` _reserveammostorage)
    (:`Is Valid`
      (bind _ammoinfo (`/Game/GenericShooter/Addons/Common/Blueprints/Interfaces/BPI_GenericAmmoStorage.GetAmmoInfoForAmmoType` _reserveammostorage AmmoType))
      (return _ammoinfo))
    (:`Is Not Valid`
      (return))))

(fn `GetUserFriendlyNameThroughInterface`
  (returns (DisplayName :type Text))
  (return (`self.FriendlyName`)))

(fn `OnFireMechanicRequestedAnimation`
  (params (FiringMechanic :type "/Game/GenericShooter/Addons/WeaponSystem/Core/BP_Weapon_FireMechanicBaseComponent Object Reference") (AnimKeyName :type Name) (StartTime :type "Float (double-precision)") (JumpToSection :type Name) (bStop :type Boolean))
  (`self.OnWeaponRequestPlayAnimation` AnimKeyName (`self.AnimWeaponCategory`) StartTime JumpToSection bStop)
  (return))

(fn `OnRep_AmmoStorageAsObject`
  (`self.PrintDebugString` (`KismetStringLibrary.Concat_StrStr` "OnRepAmmoStorageAsObject Set To: " (`KismetSystemLibrary.GetDisplayName` (`self.ReserveAmmoStorageAsObject`)))
    (:`Out`
      (bind _asbpi_generic_ammo_storage (cast `/Game/GenericShooter/Addons/Common/Blueprints/Interfaces/BPI_GenericAmmoStorage` (`self.ReserveAmmoStorageAsObject`))
        (:`then`
          (set `self.ReserveAmmoStorage` _asbpi_generic_ammo_storage))
        (:`CastFailed`
          _))
      (return))))

(fn `OnReserveAmmoChanged`
  (`self.OnVitalsChanged`)
  (return))

(fn `Reload`
  (returns (bReloaded :type Boolean))
  (locals (bAmmoReloaded :type Boolean))
  (`/Engine/EditorBlueprintResources/StandardMacros.IsValid` (`KismetSystemLibrary.Conv_InterfaceToObject` (`self.ReserveAmmoStorage`))
    (:`Is Valid`
      (if (or (`KismetSystemLibrary.IsServer`) (`KismetSystemLibrary.IsStandalone`))
        (for _array_element (`/Game/GenericShooter/Addons/WeaponSystem/Core/BP_AmmoStorageComponent.AmmoStorage` (`self.BP_AmmoStorageComponent`))
          (bind (_ammotype _currentammo _maxammo) (break `/Game/GenericShooter/Addons/WeaponSystem/Core/FWeaponAmmoStorage` _array_element))
          (bind (_bhasenoughammo _availableammo) (`/Game/GenericShooter/Addons/Common/Blueprints/Interfaces/BPI_GenericAmmoStorage.HasEnoughAmmo` (`self.ReserveAmmoStorage`) _ammotype (- _maxammo _currentammo)))
          (if (> _availableammo 0)
            (bind _ammounderflow (`/Game/GenericShooter/Addons/Common/Blueprints/Interfaces/BPI_GenericAmmoStorage.ConsumeAmmo` (`self.ReserveAmmoStorage`) _ammotype _availableammo))
            (`/Game/GenericShooter/Addons/WeaponSystem/Core/BP_AmmoStorageComponent.AddAmmo` (`self.BP_AmmoStorageComponent`) _ammotype (- _availableammo _ammounderflow) false)
            (set `local.bAmmoReloaded` true)))
        (if (`local.bAmmoReloaded`)
          (`self.OnVitalsChanged`)
          (return true)
          (else
            (return false)))
        (else
          (`self.OnVitalsChanged`)
          (return false))))
    (:`Is Not Valid`
      (return false))))

(fn `SetLoadedAmmoStorage`
  (params (AmmoStorage :type "Array of /Game/GenericShooter/Addons/WeaponSystem/Core/FWeaponAmmoStorage Structure"))
  (set `/Game/GenericShooter/Addons/WeaponSystem/Core/BP_AmmoStorageComponent.AmmoStorage` AmmoStorage (`self.BP_AmmoStorageComponent`))
  (return))

(fn `SetWeaponRecoilSpread`
  (params (HorizontalSpread :type "Float (double-precision)") (VerticalSpread :type "Float (double-precision)"))
  (`/Game/GenericShooter/Addons/WeaponSystem/Core/BP_Weapon_FireMechanicBaseComponent.SetRecoilSpreadValues` (`self.FiringMechanicComponents`) HorizontalSpread VerticalSpread)
  (return))

(fn `StartFire`
  (return))

(fn `StopFire`
  (return))

(fn `TriggerVitalsChanged`
  (`self.OnVitalsChanged`)
  (return))

(fn `UserConstructionScript`
  (`|ExecutionSequence`
    (:`then_0`
      (bind _asbpi_generic_ammo_storage (cast `/Game/GenericShooter/Addons/Common/Blueprints/Interfaces/BPI_GenericAmmoStorage` (`self.ReserveAmmoStorageAsObject`)))
      (set `self.ReserveAmmoStorage` _asbpi_generic_ammo_storage))
    (:`then_1`
      (set `self.FiringMechanicComponents` (`self.K2_GetComponentsByClass` "/Game/GenericShooter/Addons/WeaponSystem/Core/BP_Weapon_FireMechanicBaseComponent.BP_Weapon_FireMechanicBaseComponent_C")))))