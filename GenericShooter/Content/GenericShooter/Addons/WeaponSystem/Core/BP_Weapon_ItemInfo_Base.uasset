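; Base inventory item info for weapons, linking a weapon class and its pickup proxy to the inventory and carrying the weapon's loaded ammo.
; It spawns the weapon actor or a throwable world proxy, copying loaded ammo to and from the actor.
; The item bar shows the first loaded ammo type plus matching reserve as a fraction of maximum.
; An item is refused if the inventory already holds the same weapon class.
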(fn `CanBeAdded`
  (params (InventoryOwner :type "Actor Object Reference") (ExistingItems :type "Array of /Game/GenericShooter/Addons/Common/Blueprints/BaseClasses/BP_SlotInventory_ItemInfo_Base Object Reference (by ref)"))
  (returns (bCanBeAdded :type Boolean))
  (for _array_element ExistingItems
    (bind _asbp_weapon_item_info_base (cast `/Game/GenericShooter/Addons/WeaponSystem/Core/BP_Weapon_ItemInfo_Base` _array_element))
    (if (== (`/Game/GenericShooter/Addons/WeaponSystem/Core/BP_Weapon_ItemInfo_Base.WeaponClass` _asbp_weapon_item_info_base) (`self.WeaponClass`))
      (return false)))
  (return true))

(fn `GetItemBarFillPercent`
  (returns (Percent :type "Float (double-precision)"))
  (locals (TotalCurrentAmmo :type Integer) (TotalMaxAmmo :type Integer))
  (bind (_ammotype _currentammo _maxammo) (break `/Game/GenericShooter/Addons/WeaponSystem/Core/FWeaponAmmoStorage` (`|GetArrayItem` (`self.LoadedAmmoStorage`))))
  (bind (_ammotype_2 _currentammo_2 _maxammo_2) (break `/Game/GenericShooter/Addons/WeaponSystem/Core/FWeaponAmmoStorage` (`|GetArrayItem` (`self.LoadedAmmoStorage`))))
  (`self.UpdateFromActorIfInitialSpawnUsingTempActor`)
  (if (> (`KismetArrayLibrary.Array_Length` (`self.LoadedAmmoStorage`)) 0)
    (`/Engine/EditorBlueprintResources/StandardMacros.IsValid` (`KismetSystemLibrary.Conv_InterfaceToObject` (`self.ReserveAmmoStorage`))
      (:`Is Valid`
        (bind (_ammoinfo _ammoindex _bhasammoinfo) (`/Game/GenericShooter/Addons/Common/Blueprints/Interfaces/BPI_GenericAmmoStorage.GetAmmoInfoForAmmoType` (`self.ReserveAmmoStorage`) _ammotype))
        (bind (_ammotype_3 _currentammo_3 _maxammo_3) (break `/Game/GenericShooter/Addons/WeaponSystem/Core/FWeaponAmmoStorage` _ammoinfo))
        (set `local.TotalCurrentAmmo` (+ _currentammo (`KismetMathLibrary.SelectInt` _currentammo_3 0 _bhasammoinfo)))
        (set `local.TotalMaxAmmo` (+ _maxammo (`KismetMathLibrary.SelectInt` _maxammo_3 0 _bhasammoinfo)))
        (return (/ (`KismetMathLibrary.Conv_IntToDouble` (`local.TotalCurrentAmmo`)) (`KismetMathLibrary.Conv_IntToDouble` (`local.TotalMaxAmmo`)))))
      (:`Is Not Valid`
        (return (/ (`KismetMathLibrary.Conv_IntToDouble` _currentammo_2) (`KismetMathLibrary.Conv_IntToDouble` _maxammo_2)))))
    (else
      (return 0.0))))

(fn `OnRep_ReserveAmmoStorageAsObject`
  (bind _asbpi_generic_ammo_storage (cast `/Game/GenericShooter/Addons/Common/Blueprints/Interfaces/BPI_GenericAmmoStorage` (`self.ReserveAmmoStorageAsObject`))
    (:`then`
      (set `self.ReserveAmmoStorage` _asbpi_generic_ammo_storage)
      (return))
    (:`CastFailed`
      (return))))

(fn `SpawnActor`
  (params (OwningActor :type "Actor Object Reference") (Instigator :type "Pawn Object Reference") (bIsSpawningTempActor :type Boolean))
  (returns (NewActor :type "Actor Object Reference"))
  (bind _returnvalue (`|SpawnActorFromClass` (`self.WeaponClass`) (`KismetMathLibrary.MakeTransform` (0.0 0.0 0.0)) "AlwaysSpawn" "OverrideRootScale" OwningActor null Instigator))
  (`self.UpdateFromActorIfInitialSpawn` _returnvalue)
  (if (not (`local.bIsSpawningTempActor`))
    (`/Game/GenericShooter/Addons/WeaponSystem/Core/BP_Weapon_Base.SetLoadedAmmoStorage` _returnvalue (`self.LoadedAmmoStorage`))
    (return _returnvalue)
    (else
      (return _returnvalue))))

(fn `SpawnWeaponProxy`
  (params (WorldTransform :type "Transform Structure") (Owner :type "Actor Object Reference") (Instigator :type "Pawn Object Reference") (SimulatePhysics :type Boolean :default true) (ThrowVelocity :type "Vector Structure"))
  (`|SpawnActorFromClass` (`self.WeaponProxyClass`) WorldTransform "AlwaysSpawn" "OverrideRootScale" Owner self SimulatePhysics ThrowVelocity Instigator)
  (return))

(fn `UpdateFromActor`
  (params (Actor :type "Actor Object Reference"))
  (returns (bUpdated :type Boolean))
  (bind _asbp_weapon_base (cast `/Game/GenericShooter/Addons/WeaponSystem/Core/BP_Weapon_Base` Actor)
    (:`then`
      (bind _ammostorage (`/Game/GenericShooter/Addons/WeaponSystem/Core/BP_Weapon_Base.GetLoadedAmmoStorageCopy` _asbp_weapon_base))
      (set `self.LoadedAmmoStorage` _ammostorage)
      (return true))
    (:`CastFailed`
      (return false))))

(fn `UserConstructionScript`
  (`parent.UserConstructionScript`))