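; Weapon mechanic component that fires projectiles by spawning an actor of the configured projectile class.
; PerformMechanic consumes ammo, then takes the owner's aim with spread to set the spawn transform, pushed forward by an offset, and the initial velocity.
; Replicated projectile classes spawn only on server or standalone, while non-replicated ones spawn on any machine running the mechanic.
; An invalid class logs an error after ammo is already consumed.
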(event `self.PerformMechanic`
  (`self.PerformProjectileMechanic`))

(fn `PerformProjectileMechanic`
  (locals (AimLocation :type "Vector Structure") (AimRotation :type "Rotator Structure"))
  (bind (_location _rotation) (`self.GetAim`))
  (bind _output (`self.GetAimVectorWithSpread` _rotation))
  (bind (_userfriendlyname _bdebug _impacteffectclass _breplicateprojectilemovement _bexploded _bexplodeonprojectilestop _projectilestoppedimpactresult _bexplodewithimpactonpawn _initialvelocity _basedamage _minimumdamage _damageinnerradius _damageouterradius _damagefalloff _damagepreventionchannel _damagetypeclass _breplicates) (defaults `/Game/GenericShooter/Addons/WeaponSystem/Core/BP_Weapon_ProjectileComponent` (`self.ProjectileClass`)))
  (`self.ConsumeAmmo`)
  (if (`KismetSystemLibrary.IsValidClass` (`self.ProjectileClass`))
    (if (or (and _breplicates (or (`KismetSystemLibrary.IsServer`) (`KismetSystemLibrary.IsStandalone`))) (not _breplicates))
      ;[1 1 1] Get Aim Info
      (set `local.AimLocation` _location)
      (bind _output_get (set `local.AimRotation` (`KismetMathLibrary.Conv_VectorToRotator` _output)))
      (`|SpawnActorFromClass` (`self.ProjectileClass`) (`KismetMathLibrary.MakeTransform` (+ (`local.AimLocation`) (* (`KismetMathLibrary.Normal` _output) (`self.ProjectileSpawnForwardOffset`))) _output_get) "AlwaysSpawn" "OverrideRootScale" (`self.GetOwner`) _output (`self.GetOwnerOwnerAsPawn`)))
    (else
      (`VisualLoggerKismetLibrary.LogLocation` null (`Actor.K2_GetActorLocation` (`self.GetOwner`)) "Failed to fire projectile because Projectile Class is not valid!" (struct :`R` 1.0 :`B` 0.035682 :`A` 1.0))
      (return))))