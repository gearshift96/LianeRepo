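; BP_AmmoPickup_Base is the base interactable ammo pickup actor for the weapon system, showing a prompt with its amount and type.
; On interact it rejects a None type or empty amount with debug errors, then asks the interactor how much it can hold and adds that much.
; It subtracts what was added and destroys itself when emptied, or on a partial pickup if DestroyOnPartialPickup is set.
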(event `/Game/GenericShooter/Addons/Common/Blueprints/Interfaces/BPI_GenericInteractable.Interact`
  (params (Interactor :type "/Game/GenericShooter/Addons/Common/Blueprints/Interfaces/BPI_GenericInteractor Interface"))
  (bind _returnvalue (`KismetSystemLibrary.Conv_InterfaceToObject` Interactor))
  (if (`|EnumEquality` (`self.AmmoType`) "NewEnumerator3")
    (`KismetSystemLibrary.PrintString` "ERROR: Ammo pickup has an ammo type of None" true true (struct :`R` 1.0 :`A` 1.0))
    (elif (<= (`self.AmmoAmount`) 0)
      (`KismetSystemLibrary.PrintString` "ERROR: Ammo pickup has no ammo to pickup." true true (struct :`R` 1.0 :`A` 1.0))
      (else
        (bind _amounttopickup (message `/Game/GenericShooter/Addons/Common/Blueprints/Interfaces/BPI_WeaponSystem_Holder.CanHoldMoreWeaponAmmo` _returnvalue (`self.AmmoType`) (`self.AmmoAmount`)))
        (if (> _amounttopickup 0)
          (bind (_baddedammo _amountadded) (message `/Game/GenericShooter/Addons/Common/Blueprints/Interfaces/BPI_WeaponSystem_Holder.AddWeaponAmmo` _returnvalue (`self.AmmoType`) _amounttopickup))
          (bind _output_get (set `self.AmmoAmount` (- (`self.AmmoAmount`) _amountadded)))
          (if (or (and (> _output_get 0) (`self.bDestroyOnPartialPickup`)) (<= _output_get 0))
            (set `self.AmmoAmount` 0)
            (`self.K2_DestroyActor`)))))))

(fn `GetDesiredHeldRotation`
  (returns (RelativeHeldRotation :type "Rotator Structure"))
  (return))

(fn `GetInteractionCenterPoint`
  (returns (WorldLocation :type "Vector Structure"))
  (return (0.0 0.0 0.0)))

(fn `GetInteractionText`
  (params (Interactor :type "/Game/GenericShooter/Addons/Common/Blueprints/Interfaces/BPI_GenericInteractor Interface"))
  (returns (Text :type Text))
  (return (`|FormatText` "Pickup {Amount} {AmmoType} Ammo" (`self.AmmoAmount`) (`KismetTextLibrary.Conv_StringToText` (`|GetEnumeratorNameAsString` (`self.AmmoType`))))))

(fn `IsFocusable`
  (params (Interactor :type "/Game/GenericShooter/Addons/Common/Blueprints/Interfaces/BPI_GenericInteractor Interface"))
  (returns (bFocusable :type Boolean))
  (return true))

(fn `IsPhysicsPickup`
  (returns (bPickupable :type Boolean) (PickupComponent :type "PrimitiveComponent Object Reference"))
  (return false null))

(fn `ShouldNotInteractOnClients`
  (returns (bShouldNotInteractOnClients :type Boolean))
  (return false))

(fn `ShouldNotSendInteractToServer`
  (returns (bShouldNotSendInteractToServer :type Boolean))
  (return false))

(fn `UserConstructionScript`)