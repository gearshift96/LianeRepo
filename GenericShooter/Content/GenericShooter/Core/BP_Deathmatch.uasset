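; Deathmatch game mode that forces a single team and ends the match when a kill limit is won.
; BeginPlay parses options for kill limit, player cap and LAN, attempts session creation on multiplayer servers, and hooks up the lobby manager.
; Spawning favors random unoccupied valid starts, with encroached or optional native fallback, and binds pawn health pre-death events for kill checks.
; Match state, restart, death and winner logic delegate to shared Example helper functions.
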(event `self.ReceiveBeginPlay`
  ;[0 0.0652 1] @GenericPlatformTools: Delete this node and call it in ConfigureGameSettings (Choose Override instead of New Function to find ConfigureGameSettings)
  (`self.SetGameOptions` (`self.OptionsString`))
  (`self.EnsureCreateSessionAttempted`)
  ;[1 1 1] Update our replicated game mode display name once a game state is available
  (`/Game/GenericShooter/Addons/MatchLobby/Core/BP_LobbyManagerComponent.SetGameModeDescription` (`self.GetComponentByClass` (`GameplayStatics.GetGameState`) "/Game/GenericShooter/Addons/MatchLobby/Core/BP_LobbyManagerComponent.BP_LobbyManagerComponent_C") (`self.GameModeDisplayName`))
  (bind _lobbymanager (`/Game/GenericShooter/Addons/MatchLobby/Core/BPFL_LobbyManager.GetLobbyManagerFromGameStateImpure`))
  (add `/Game/GenericShooter/Addons/MatchLobby/Core/BP_LobbyManagerComponent.OnShouldAnnounceWinner` _lobbymanager (delegate `AnnounceWinner`)))

(event `AnnounceWinner`
  (`/Game/GenericShooter/Core/BPFL_GenericShooterExampleLogic.ExampleAnnounceWinner`))

(event `self.K2_OnSetMatchState`
  (params (NewState :type Name))
  ;[1 1 1] Forward match state changes to our lobby manager
  (`/Game/GenericShooter/Core/BPFL_GenericShooterExampleLogic.ExampleOnSetMatchState` NewState))

(event `self.HandleStartingNewPlayer`
  (params (NewPlayer :type "PlayerController Object Reference"))
  ;[1 1 1] Handle starting of a new player
  (`/Game/GenericShooter/Core/BPFL_GenericShooterExampleLogic.ExampleOnHandleStartingNewPlayer` NewPlayer))

(event `EnsureCreateSessionAttempted`
  ;[1 1 1] Ensure they we've tried registering our server if multiplayer with our platform service. This could fail if a session was already created, which can happen if a user creates a server through the UI instead of launching a server on the command line or using a dedicated server.
  (if (and (`KismetSystemLibrary.IsServer`) (not (`KismetSystemLibrary.IsStandalone`)))
    (`CreateSessionCallbackProxy.CreateSession` (`GameplayStatics.GetPlayerController` 0) (`self.CurrentMaxPlayers`) (`self.bLanOnlyDesired`)
      (:`OnSuccess`
        (`KismetSystemLibrary.PrintString` "Server successfully auto-created a session." false true (struct :`G` 1.0 :`B` 0.086407 :`A` 1.0))))))

(fn `BPCallablePlayerCanRestart`
  (params (Player :type "PlayerController Object Reference"))
  (returns (bCanRestart :type Boolean))
  (bind _bcanrestart (`/Game/GenericShooter/Core/BPFL_GenericShooterExampleLogic.ExamplePlayerCanRestart` Player))
  (return _bcanrestart))

(fn `ChoosePlayerStart`
  (params (Player :type "Controller Object Reference"))
  (returns (ReturnValue :type "Actor Object Reference"))
  (locals (UnencroachedPlayerStarts :type "Array of PlayerStart Object Reference") (EncroachedPlayerStarts :type "Array of PlayerStart Object Reference") (TestTeamNum :type Byte))
  (bind _encroachedplayerstarts (`local.EncroachedPlayerStarts`))
  (bind _unencroachedplayerstarts (`local.UnencroachedPlayerStarts`))
  (`|ExecutionSequence`
    (:`then_0`
      ;[1 1 1] Assemble a list of all valid spawn points
      (bind _outactors (`GameplayStatics.GetAllActorsOfClass` "/Game/GenericShooter/Core/BP_GenericPlayerStart.BP_GenericPlayerStart_C"))
      (for _array_element _outactors
        (if (`/Game/GenericShooter/Core/BP_GenericPlayerStart.IsValidSpawnPointForController` _array_element (`local.Player`))
          (if (`/Game/GenericShooter/Core/BP_GenericPlayerStart.IsPawnAtSpawn` _array_element)
            (`KismetArrayLibrary.Array_Add` (`local.EncroachedPlayerStarts`))
            (else
              (`KismetArrayLibrary.Array_Add` (`local.UnencroachedPlayerStarts`) _array_element))))))
    (:`then_1`
      ;[1 1 1] Grab an unencroached start if possible
      (if (`KismetArrayLibrary.Array_IsValidIndex` _unencroachedplayerstarts)
        (return (`|GetArrayItem` _unencroachedplayerstarts (`KismetMathLibrary.RandomIntegerInRange` 0 (- (`KismetArrayLibrary.Array_Length` _unencroachedplayerstarts) 1))))
        (else
          ;[1 1 1] If no unencroached exist, fall back to encroached starts
          (if (`KismetArrayLibrary.Array_IsValidIndex` _encroachedplayerstarts)
            (return (`|GetArrayItem` _encroachedplayerstarts (`KismetMathLibrary.RandomIntegerInRange` 0 (- (`KismetArrayLibrary.Array_Length` _encroachedplayerstarts) 1))))
            (else
              ;[1 1 1] If failed to find player start, fall back to native behavior or return null
              (if (`self.bFallbackToNativePlayerStart`)
                (bind _returnvalue (`parent.ChoosePlayerStart` (`local.Player`)))
                (return _returnvalue)
                (else
                  (return null))))))))))

(fn `OnPawnDied`
  (params (DeadActor :type "Actor Object Reference") (OverkillDamage :type "Float (double-precision)"))
  (locals (DeadPawn :type "Pawn Object Reference") (DeadPlayerState :type "PlayerState Object Reference") (KillerPlayerState :type "PlayerState Object Reference") (DamageCauserDisplayName :type Text) (DeadHealthComponent :type "/Game/GenericShooter/Addons/HealthComponent/Core/BP_HealthComponent Object Reference"))
  (bind _aspawn (cast `Pawn` DeadActor)
    (:`then`
      (`/Game/GenericShooter/Core/BPFL_GenericShooterExampleLogic.ExampleServerHandleCharacterDied` _aspawn)
      (bind (_bgamewon _winningteamnum _highestrankedonwinningteam) (`/Game/GenericShooter/Core/BPFL_GenericShooterExampleLogic.ExampleCheckForKillLimitWinner` (`self.KillLimit`)))
      (if _bgamewon
        (`/Game/GenericShooter/Core/BPFL_GenericShooterExampleLogic.ExampleEndMatchWithWinner` _highestrankedonwinningteam)
        (return)
        (else
          (return))))
    (:`CastFailed`
      (return))))

(fn `PlayerCanRestart`
  (params (Player :type "PlayerController Object Reference"))
  (returns (ReturnValue :type Boolean))
  (bind _bcanrestart (`/Game/GenericShooter/Core/BPFL_GenericShooterExampleLogic.ExamplePlayerCanRestart` Player))
  (return _bcanrestart))

(fn `ReadyToEndMatch`
  (returns (ReturnValue :type Boolean))
  (bind _breadytoendmatch (`/Game/GenericShooter/Core/BPFL_GenericShooterExampleLogic.ExampleReadyToEndMatch`))
  (return _breadytoendmatch))

(fn `ReadyToStartMatch`
  (returns (ReturnValue :type Boolean))
  (bind _breadytostartmatch (`/Game/GenericShooter/Core/BPFL_GenericShooterExampleLogic.ExampleReadyToStartMatch`))
  (return _breadytostartmatch))

(fn `SetGameOptions`
  (params (Options :type String))
  (returns (bSet :type Boolean))
  (`|ExecutionSequence`
    (:`then_0`
      ;[1 1 1] Pass along config settings, but then force Num Teams to be 1 since we're in deathmatch
      (`/Game/GenericShooter/Core/BPFL_GenericShooterExampleLogic.ExampleSetGameStateOptions` (`local.Options`))
      (`/Game/GenericShooter/Addons/TeamManager/Core/BP_TeamManagerComponent.SetNumTeams` (`self.GetComponentByClass` (`GameplayStatics.GetGameState`) "/Game/GenericShooter/Addons/TeamManager/Core/BP_TeamManagerComponent.BP_TeamManagerComponent_C") 1))
    (:`then_1`
      ;[1 1 1] Kill Limit
      (set `self.KillLimit` (`GameplayStatics.GetIntOption` (`local.Options`) (`self.KillLimitKey`) (`self.KillLimit`))))
    (:`then_2`
      ;[1 1 1] Set Current Max Players
      (set `self.CurrentMaxPlayers` (`GameplayStatics.GetIntOption` (`local.Options`) (`self.CurrentMaxPlayersKey`) (`self.MaxPlayers`))))
    (:`then_3`
      ;[1 1 1] Set Lan Only Desired
      (set `self.bLanOnlyDesired` (`GameplayStatics.HasOption` (`local.Options`) (`self.LanOnlyKey`))))
    (:`then_4`
      (return true))))

(fn `SpawnDefaultPawnAtTransform`
  (params (NewPlayer :type "Controller Object Reference") (SpawnTransform :type "Transform Structure (by ref)"))
  (returns (ReturnValue :type "Pawn Object Reference"))
  (bind _returnvalue (`|SpawnActorFromClass` (`self.DefaultPawnClass`) SpawnTransform "Undefined" "OverrideRootScale" null (`self.GetInstigator`)))
  (`/Engine/EditorBlueprintResources/StandardMacros.IsValid` _returnvalue
    (:`Is Valid`
      (bind _returnvalue_2 (`self.GetComponentByClass` _returnvalue "/Game/GenericShooter/Addons/HealthComponent/Core/BP_HealthComponent.BP_HealthComponent_C"))
      (`/Engine/EditorBlueprintResources/StandardMacros.IsValid` _returnvalue_2
        (:`Is Valid`
          (add `/Game/GenericShooter/Addons/HealthComponent/Core/BP_HealthComponent.OnServerPreDeath` _returnvalue_2 (`|CreateDelegate` :!event `OnPawnDied`)))
        (:`Is Not Valid`
          _)))
    (:`Is Not Valid`
      _))
  (return _returnvalue))

(fn `UserConstructionScript`
  (`parent.UserConstructionScript`))