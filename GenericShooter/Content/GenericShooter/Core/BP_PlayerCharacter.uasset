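; Networked player character for a shooter, routing input for movement, camera, interaction and weapons to components for health, inventory, weapon handling, ammo and skins.
; The server grants default weapons, spawns the equipped one and handles throwing it as a pickup proxy.
; Inventory selection drives switching: holster the current weapon, then server-spawn the desired one from its item info.
; It also handles team-based materials, match-end shutdown and timed cleanup after unpossession.
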(event `self.ReceiveTick`
  (params (DeltaSeconds :type "Float (single-precision)"))
  ;[1 1 1] @TODO: Move updating name tags out of tick
  (`/Game/GenericShooter/Core/BPFL_GenericShooterExampleLogic.ExampleUpdatePawnNameTag` (`self.NameTag`) true true false false (struct :`R` 0.085431 :`G` 1.0 :`A` 1.0) (struct :`R` 1.0 :`A` 1.0) true))

(event `self.ReceiveDestroyed`
  ;[1 0.2855 0 0.069] Destruction
)

(event `self.ReceiveBeginPlay`
  (bind _returnvalue (`self.GetComponentByClass` (`GameplayStatics.GetGameState`) "/Game/GenericShooter/Addons/MatchLobby/Core/BP_LobbyManagerComponent.BP_LobbyManagerComponent_C"))
  ;[0 1 0.101 0.137] On Spawn...
  (`self.BindWeaponComponents`)
  (`self.SetUpNetworkingBehavior`)
  ;;[1 1 1] If we're on the server, spawn us our default weapons. These weapons will be replicated.
  (`self.GiveDefaultWeapons`)
  ;[1 1 1] Stop doing things when match ends
  (add `/Game/GenericShooter/Addons/MatchLobby/Core/BP_LobbyManagerComponent.OnMatchEndSummary` _returnvalue (delegate `StopDoingThingsOnMatchEnd`))
  (add `/Game/GenericShooter/Addons/MatchLobby/Core/BP_LobbyManagerComponent.OnMatchWaitingPostMatch` _returnvalue (delegate `StopDoingThingsOnMatchEnd`)))

(event `StopDoingThingsOnMatchEnd`
  ;[1 1 1] Stop doing things when match ends
  (`/Engine/EditorBlueprintResources/StandardMacros.DoOnce` false
    (:`Completed`
      (`/Game/GenericShooter/Core/BPFL_GenericShooterExampleLogic.ExampleHandlePawnMatchEnd` self))))

(event `Key|PageDown`
  (params (Key :type "Key Structure"))
  ;[1 1 1] Debug Skin Keys
  (:`Pressed`
    (`/Game/GenericShooter/Addons/Skinner/Core/BP_SkinnerComponent.ChangeCharacterSkin` (`self.BP_BasicSkinnerComponent`) "Default" true false)))

(event `self.OnLanded`
  (params (Hit :type "HitResult Structure (by ref)"))
  ;[0.9774 1 0 0.183] Damage
  ;;[1 1 1] On the server only, handle damage logic. Resulting Health gets replicated to clients
  (`/Game/GenericShooter/Addons/HealthComponent/Core/BP_HealthComponent.ConsiderFallDamageOnLand` (`self.BP_HealthComponent`) Hit))

(event `self.BP_HealthComponent.OnDied`
  (params (DeadActor :type "Actor Object Reference") (OverkillDamage :type "Float (single-precision)"))
  ;[0.9774 1 0 0.183] Damage
  (`/Game/GenericShooter/Core/BPFL_GenericShooterExampleLogic.ExampleHandlePawnDied` self))

(event `Key|PageUp`
  (params (Key :type "Key Structure"))
  ;[1 1 1] Debug Skin Keys
  (:`Pressed`
    (`/Game/GenericShooter/Addons/Skinner/Core/BP_SkinnerComponent.ChangeCharacterSkin` (`self.BP_BasicSkinnerComponent`) "IBCardboard" true false)))

(event `self.BP_CharacterWeaponManagementComponent.OnThrowFinished`
  (bind (_worldtransform _throwvector) (`self.GetWeaponThrowTransformAndForce`))
  (bind _gameplayactiveitem (`/Game/GenericShooter/Addons/SlotInventory/Core/BP_SlotInventoryComponent.GameplayActiveItem` (`self.BP_WIComponent`)))
  (`/Engine/EditorBlueprintResources/ActorMacros.Switch Has Authority`
    (:`Authority`
      (bind _asbp_weapon_item_info_base (cast `/Game/GenericShooter/Addons/WeaponSystem/Core/BP_Weapon_ItemInfo_Base` _gameplayactiveitem))
      (`/Game/GenericShooter/Addons/WeaponSystem/Core/BP_Weapon_ItemInfo_Base.SpawnWeaponProxy` _asbp_weapon_item_info_base _worldtransform null self true _throwvector)
      (`/Game/GenericShooter/Addons/SlotInventory/Core/BP_SlotInventoryComponent.RemoveItem` (`self.BP_WIComponent`) _gameplayactiveitem false)
      (bind _asbp_weapon_item_info_base_2 (cast `/Game/GenericShooter/Addons/WeaponSystem/Core/BP_Weapon_ItemInfo_Base` (`/Game/GenericShooter/Addons/SlotInventory/Core/BP_SlotInventoryComponent.GetHighestPriorityItemInLowestSlot` (`self.BP_WIComponent`) "/Game/GenericShooter/Addons/WeaponSystem/Core/BP_Weapon_ItemInfo_Base.BP_Weapon_ItemInfo_Base_C")))
      (set `/Game/GenericShooter/Addons/SlotInventory/Core/BP_SlotInventoryComponent.GameplayActiveItem` _asbp_weapon_item_info_base_2 (`self.BP_WIComponent`))
      (set `self.DesiredWeaponInfo` _asbp_weapon_item_info_base_2)
      (`self.SpawnAndEquipDesiredWeapon`))))

(event `self.BP_BasicSkinnerComponent.OnSkinApplied`
  (params (CharacterKeyName :type Name))
  (`self.UpdateSkinnerParameters`))

(event `InputAction|SwitchToPrimary`
  (params (Key :type "Key Structure"))
  ;[0 0 0] Weapon Input Handling
  ;;[1 1 1] Handle weapon switching
  (:`Pressed`
    (`/Game/GenericShooter/Addons/SlotInventory/Core/BP_SlotInventoryComponent.AttemptSwitchToSlot` (`self.BP_WIComponent`) 0 null false)))

(event `InputAction|Fire`
  (params (Key :type "Key Structure"))
  (bind _bp_characterweaponmanagementcomponent (`self.BP_CharacterWeaponManagementComponent`))
  (bind _bisalive (`/Game/GenericShooter/Addons/HealthComponent/Core/BP_HealthComponent.IsAlive` (`self.BP_HealthComponent`)))
  ;[0 0 0] Weapon Input Handling
  ;;[1 1 1] Fire Handling
  (:`Pressed`
    (if _bisalive :!label _label
      (bind _bshouldconsume (`/Game/GenericShooter/Addons/SlotInventory/Core/BP_SlotInventoryComponent.CommitToSelected` (`self.BP_WIComponent`)))
      (if (not _bshouldconsume)
        (`/Game/GenericShooter/Addons/WeaponSystem/Core/BP_CharacterWeaponManagementComponent.StartFire` _bp_characterweaponmanagementcomponent))))
  (:`Released`
    (if _bisalive :!label _label_2
      (`/Game/GenericShooter/Addons/WeaponSystem/Core/BP_CharacterWeaponManagementComponent.StopFire` _bp_characterweaponmanagementcomponent))))

(event `InputAxis|MoveForward`
  (params (AxisValue :type "Float (single-precision)"))
  ;[0 0 0] Basic Input Handling
  ;;[1 1 1] Movement Handling
  (`self.AddMovementInput` (`SceneComponent.GetForwardVector` (`self.CapsuleComponent`)) AxisValue))

(event `InputAction|Jump`
  (params (Key :type "Key Structure"))
  ;[0 0 0] Basic Input Handling
  ;;[1 1 1] Handle Jumping
  (:`Pressed`
    (`self.Jump`)))

(event `EditorFire`
  ;[0 0 0] Weapon Input Handling
  ;;[1 1 1] Fire Handling
  (goto _label))

(event `InputAction|SwitchToSecondary`
  (params (Key :type "Key Structure"))
  ;[0 0 0] Weapon Input Handling
  ;;[1 1 1] Handle weapon switching
  (:`Pressed`
    (`/Game/GenericShooter/Addons/SlotInventory/Core/BP_SlotInventoryComponent.AttemptSwitchToSlot` (`self.BP_WIComponent`) 1 null false)))

(event `EditorStopFire`
  ;[0 0 0] Weapon Input Handling
  ;;[1 1 1] Fire Handling
  (goto _label_2))

(event `InputAxis|MoveRight`
  (params (AxisValue :type "Float (single-precision)"))
  ;[0 0 0] Basic Input Handling
  ;;[1 1 1] Movement Handling
  (`self.AddMovementInput` (`SceneComponent.GetRightVector` (`self.CapsuleComponent`)) AxisValue))

(event `InputAction|SwitchToSpecial`
  (params (Key :type "Key Structure"))
  ;[0 0 0] Weapon Input Handling
  ;;[1 1 1] Handle weapon switching
  (:`Pressed`
    (`/Game/GenericShooter/Addons/SlotInventory/Core/BP_SlotInventoryComponent.AttemptSwitchToSlot` (`self.BP_WIComponent`) 2 null false)))

(event `InputAction|Reload`
  (params (Key :type "Key Structure"))
  ;[0 0 0] Weapon Input Handling
  ;;[1 1 1] Reload Handling
  (:`Pressed`
    (`/Game/GenericShooter/Addons/WeaponSystem/Core/BP_CharacterWeaponManagementComponent.StartReload` (`self.BP_CharacterWeaponManagementComponent`))))

(event `InputAxis|LookUp`
  (params (AxisValue :type "Float (single-precision)"))
  ;[0 0 0] Basic Input Handling
  ;;[1 1 1] Turn Handling
  (`self.AddControllerPitchInput` (* (* AxisValue (`KismetMathLibrary.SelectFloat` -1.0 1.0 (`self.bInvertY`))) (`self.AimSensitivity`))))

(event `InputAction|Aim`
  (params (Key :type "Key Structure"))
  (bind _bp_characterweaponmanagementcomponent (`self.BP_CharacterWeaponManagementComponent`))
  ;[0 0 0] Weapon Input Handling
  ;;[1 1 1] Handle Aiming Down Sight
  (:`Pressed`
    (`/Game/GenericShooter/Addons/WeaponSystem/Core/BP_CharacterWeaponManagementComponent.StartADS` _bp_characterweaponmanagementcomponent))
  (:`Released`
    (`/Game/GenericShooter/Addons/WeaponSystem/Core/BP_CharacterWeaponManagementComponent.StopADS` _bp_characterweaponmanagementcomponent)))

(event `InputAxis|LookRight`
  (params (AxisValue :type "Float (single-precision)"))
  ;[0 0 0] Basic Input Handling
  ;;[1 1 1] Turn Handling
  (`self.AddControllerYawInput` (* AxisValue (`self.AimSensitivity`))))

(event `InputAction|DropWeapon`
  (params (Key :type "Key Structure"))
  ;[0 0 0] Weapon Input Handling
  ;;[1 1 1] Handle dropping weapon
  (:`Pressed`
    (`/Game/GenericShooter/Addons/WeaponSystem/Core/BP_CharacterWeaponManagementComponent.StartThrow` (`self.BP_CharacterWeaponManagementComponent`))))

(event `InputAction|Crouch`
  (params (Key :type "Key Structure"))
  (bind _btogglecrouch (`self.bToggleCrouch`))
  ;[0 0 0] Game Logic Specific Character Input Handling
  ;;[1 1 1] Handle Pawn Crouching
  (:`Pressed`
    (if _btogglecrouch
      (`/Engine/EditorBlueprintResources/StandardMacros.FlipFlop`
        (:`A`
          (`self.Crouch` :!label _label_3))
        (:`B`
          (`self.UnCrouch` :!label _label_4)))
      (else
        (goto _label_3))))
  (:`Released`
    (if (not _btogglecrouch)
      (goto _label_4))))

(event `InputAction|ToggleCamera`
  (params (Key :type "Key Structure"))
  (bind _bp_charactercameramanagercomponent (`self.BP_CharacterCameraManagerComponent`))
  ;[0 0 0] Camera Input Handling
  (:`Pressed`
    (switch `name` (`/Game/GenericShooter/Addons/CharacterCameraManager/Core/BP_CharacterCameraManagerComponent.GetActiveCameraName` _bp_charactercameramanagercomponent)
      (:`ThirdPerson`
        (`/Game/GenericShooter/Addons/CharacterCameraManager/Core/BP_CharacterCameraManagerComponent.SetActiveCamera` _bp_charactercameramanagercomponent "FirstPerson"))
      (:`FirstPerson`
        (`/Game/GenericShooter/Addons/CharacterCameraManager/Core/BP_CharacterCameraManagerComponent.SetActiveCamera` _bp_charactercameramanagercomponent "ThirdPerson")))))

(event `InputAction|Interact`
  (params (Key :type "Key Structure"))
  ;[0 0 0] Interaction Input Handling
  ;;[1 1 1] Handle Pawn interactions with pickupables
  (:`Pressed`
    (`/Engine/EditorBlueprintResources/ActorMacros.Switch Has Authority`
      (:`Authority`
        (`/Game/GenericShooter/Addons/Interaction/Core/BP_GenericInteractionComponent.Interact` (`self.BP_GenericInteractionComponent`) :!label _label_5))
      (:`Remote`
        (`self.ServerInteract`)))))

(event `ServerInteract`
  ;[0 0 0] Interaction Input Handling
  ;;[1 1 1] Handle Pawn interactions with pickupables
  (goto _label_5))

(event `self.ReceiveUnpossessed`
  (params (OldController :type "Controller Object Reference"))
  ;[1 1 1] Destroy pawns after configured time so they don't linger forever
  (`/Game/GenericShooter/Addons/WeaponSystem/Core/BP_CharacterWeaponManagementComponent.StopFire` (`self.BP_CharacterWeaponManagementComponent`))
  (`self.SetLifeSpan` (`self.UnpossessedLifeSpan`)))

(event `self.ReceivePossessed`
  (params (NewController :type "Controller Object Reference"))
  ;[1 1 1] Make sure if we are possessed we don't delete ourselves due to Unpossessed timer. Also a good time to update visuals.
  (`self.SetLifeSpan` 0.0)
  (bind _asplayer_controller (cast `PlayerController` NewController))
  (`PlayerController.SetViewTargetWithBlend` _asplayer_controller self 0.0 "VTBlend_Linear" 0.0 false))

(event `OnMatchEnded`
  ;[1 1 1] On match end, disable movement and activate hero cams
  (`/Game/GenericShooter/Addons/WeaponSystem/Core/BP_CharacterWeaponManagementComponent.StopFire` (`self.BP_CharacterWeaponManagementComponent`))
  (bind _asplayer_controller (cast `PlayerController` (`self.GetController`))
    (:`then`
      (`self.DisableInput` _asplayer_controller))
    (:`CastFailed`
      _))
  (`CharacterMovementComponent.DisableMovement` (`self.CharacterMovement`)))

(event `ServerSwitchToWeapon`
  (params (DesiredWeaponInfo :type "/Game/GenericShooter/Addons/WeaponSystem/Core/BP_Weapon_ItemInfo_Base Object Reference"))
  (bind _bp_characterweaponmanagementcomponent (`self.BP_CharacterWeaponManagementComponent`))
  (set `self.DesiredWeaponInfo` DesiredWeaponInfo)
  (`/Engine/EditorBlueprintResources/StandardMacros.IsValid` (`/Game/GenericShooter/Addons/WeaponSystem/Core/BP_CharacterWeaponManagementComponent.Weapon` _bp_characterweaponmanagementcomponent)
    (:`Is Valid`
      (`/Game/GenericShooter/Addons/WeaponSystem/Core/BP_CharacterWeaponManagementComponent.HolsterWeapon` _bp_characterweaponmanagementcomponent false))
    (:`Is Not Valid`
      (`self.DebugPrintWeaponLogic` "Not holding a weapon, performing fast equip."
        (:`Out`
          (`self.SpawnAndEquipDesiredWeapon`))))))

(event `self.BP_CharacterWeaponManagementComponent.OnWeaponVitalsChanged`
  (params (Weapon :type "/Game/GenericShooter/Addons/WeaponSystem/Core/BP_Weapon_Base Object Reference"))
  (bind _gameplayactiveitem (`/Game/GenericShooter/Addons/SlotInventory/Core/BP_SlotInventoryComponent.GameplayActiveItem` (`self.BP_WIComponent`)))
  (`/Engine/EditorBlueprintResources/StandardMacros.IsValid` _gameplayactiveitem
    (:`Is Valid`
      (`/Game/GenericShooter/Addons/Common/Blueprints/BaseClasses/BP_SlotInventory_ItemInfo_Base.UpdateFromActor` _gameplayactiveitem Weapon))
    (:`Is Not Valid`
      (`self.DebugPrintWeaponLogic` "Weapon Vitals Changed Without A Gameplay Active Item"))))

(event `self.BP_AmmoStorageComponent.OnAmmoChanged`
  (`/Game/GenericShooter/Addons/WeaponSystem/Core/BP_CharacterWeaponManagementComponent.TellWeaponReserveAmmoChanged` (`self.BP_CharacterWeaponManagementComponent`)))

(fn `AddWeaponAmmo`
  (params (AmmoType :type "/Game/GenericShooter/Addons/WeaponSystem/Core/EWeaponAmmoType Enum" :default "NewEnumerator3") (Amount :type Integer))
  (returns (bAddedAmmo :type Boolean) (AmountAdded :type Integer))
  (bind _ammoadded (`/Game/GenericShooter/Addons/WeaponSystem/Core/BP_AmmoStorageComponent.AddAmmo` (`self.BP_AmmoStorageComponent`) AmmoType Amount false))
  (return (> _ammoadded 0) _ammoadded))

(fn `BindWeaponComponents`
  (add `/Game/GenericShooter/Addons/SlotInventory/Core/BP_SlotInventoryComponent.OnItemSelected` (`self.BP_WIComponent`) (`|CreateDelegate` :!event `OnItemInfoSelected`))
  (add `/Game/GenericShooter/Addons/WeaponSystem/Core/BP_CharacterWeaponManagementComponent.OnHolsterFinished` (`self.BP_CharacterWeaponManagementComponent`) (`|CreateDelegate` :!event `OnHolsterFinished`))
  (return))

(fn `CanHoldMoreWeaponAmmo`
  (params (AmmoType :type "/Game/GenericShooter/Addons/WeaponSystem/Core/EWeaponAmmoType Enum" :default "NewEnumerator3") (amount :type Integer))
  (returns (AmountToPickup :type Integer))
  (bind (_bcanholdmoreammo _bcanholdallammo _canholdamount) (`/Game/GenericShooter/Addons/WeaponSystem/Core/BP_AmmoStorageComponent.CanHoldMoreAmmo` (`self.BP_AmmoStorageComponent`) AmmoType amount))
  (return _canholdamount))

(fn `CanThrowCurrentWeapon`
  (returns (bCanThrow :type Boolean))
  (bind (_items _num) (`/Game/GenericShooter/Addons/SlotInventory/Core/BP_SlotInventoryComponent.GetItemsOfClass` (`self.BP_WIComponent`) "/Game/GenericShooter/Addons/WeaponSystem/Core/BP_Weapon_ItemInfo_Base.BP_Weapon_ItemInfo_Base_C"))
  (return (> _num 1)))

(fn `CanToggleCamera`
  (returns (CanToggle :type Boolean))
  ;[1 1 1] If this ever returns false, camera switching will be blocked
  (return (and (not false) (not false))))

(fn `EdGraph_704`
  (params (TeamNum :type Byte))
  (returns (NewTeamNum :type Byte))
  (bind _output_get (set `self.TeamNum` TeamNum))
  (return _output_get))

(fn `GetCastedController`
  (returns (OutController :type "/Game/GenericShooter/Core/BP_PlayerController Object Reference") (IsValid :type Boolean))
  (bind (_asbp_player_controller _bsuccess) (cast `/Game/GenericShooter/Core/BP_PlayerController` (`self.GetController`) :!pure true))
  ;[1 1 1] Helper function that grabs a casted version of our player controller for us
  (return _asbp_player_controller _bsuccess))

(fn `GetEyeLocation`
  (returns (EyeLocation :type "Vector Structure"))
  ;[1 1 1] Get this Pawn's Eye location, which might not match our camera's location (i.e. thirdperson doesn't view from eyes)
  (return (+ (`SceneComponent.K2_GetComponentLocation` (`self.CapsuleComponent`)) (`KismetMathLibrary.MakeVector` 0.0 0.0 (`KismetMathLibrary.SelectFloat` (`self.CrouchedEyeHeight`) (`self.BaseEyeHeight`) (`NavMovementComponent.IsCrouching`))))))

(fn `GetFocusedInteractable`
  (returns (Interactable :type "/Game/GenericShooter/Addons/Common/Blueprints/Interfaces/BPI_GenericInteractable Interface") (bIsValid :type Boolean))
  (return null false))

(fn `GetInteractionCollider`
  (returns (Collider :type "PrimitiveComponent Object Reference"))
  (return null))

(fn `GetInteractionIgnoreList`
  (returns (ActorsToIgnore :type "Array of Actor Object Reference"))
  (return (`|MakeArray`)))

(fn `GetInteractionTraceLine`
  (returns (StartPoint :type "Vector Structure") (AimDirection :type "Vector Structure"))
  (return (0.0 0.0 0.0) (0.0 0.0 0.0)))

(fn `GetPhysicsHandle`
  (returns (PhysicsHandleComponent :type "PhysicsHandleComponent Object Reference"))
  (return null))

(fn `GetPhysicsHandleTargetLocationAndRotation`
  (returns (HandleLocation :type "Vector Structure") (HandleRotation :type "Rotator Structure"))
  (bind _physicshandlelocation (`self.PhysicsHandleLocation`))
  (return (`SceneComponent.K2_GetComponentLocation` _physicshandlelocation) (`SceneComponent.K2_GetComponentRotation` _physicshandlelocation)))

(fn `GetScoreForRanking`
  (returns (Score :type "Float (double-precision)"))
  (bind _playerstate (`self.PlayerState`)
    (:`then`
      (bind _score (message `/Game/GenericShooter/Addons/Common/Blueprints/Interfaces/BPI_TeamMember.GetScoreForRanking` _playerstate))
      (return _score))
    (:`else`
      (return 0.0))))

(fn `GetShouldUseThirdPersonForFireEffects`
  (returns (bThirdPerson :type Boolean))
  (return (or (not (`self.IsLocallyControlled`)) (`/Game/GenericShooter/Addons/CharacterCameraManager/Core/BP_CharacterCameraManagerComponent.IsInThirdPerson` (`self.BP_CharacterCameraManagerComponent`)))))

(fn `GetTeamNum`
  (returns (TeamNum :type Byte))
  (bind _teamnum (message `/Game/GenericShooter/Addons/Common/Blueprints/Interfaces/BPI_TeamMember.GetTeamNum` (`self.PlayerState`)))
  (return _teamnum))

(fn `GetWeaponAnimCharacterCategory`
  (returns (CharacterCategory :type Name))
  (return (`/Game/GenericShooter/Addons/Skinner/Core/BP_SkinnerComponent.CharacterAnimSetName` (`self.BP_BasicSkinnerComponent`))))

(fn `GetWeaponCrosshairVisibility`
  (returns (bVisibile :type Boolean))
  (return (and (`/Game/GenericShooter/Addons/WeaponSystem/Core/BP_CharacterWeaponManagementComponent.GetWeaponCrosshairVisibility` (`self.BP_CharacterWeaponManagementComponent`)) (`self.IsAlive`))))

(fn `GetWeaponThrowTransformAndForce`
  (returns (WorldTransform :type "Transform Structure") (ThrowVector :type "Vector Structure"))
  (bind _returnvalue (`self.GetControlRotation`))
  (bind _throwforce (`self.ThrowForce`))
  (bind _physicshandlelocation (`self.PhysicsHandleLocation`))
  (bind _returnvalue_2 (`KismetMathLibrary.GetForwardVector` _returnvalue))
  (if (`/Game/GenericShooter/Addons/CharacterCameraManager/Core/BP_CharacterCameraManagerComponent.IsInThirdPerson` (`self.BP_CharacterCameraManagerComponent`))
    (return (`SceneComponent.K2_GetComponentToWorld` _physicshandlelocation) (+ (* (`SceneComponent.GetForwardVector` _physicshandlelocation) _throwforce) (`KismetMathLibrary.MakeVector` 0.0 0.0 (/ _throwforce 4.0))))
    (else
      (return (`KismetMathLibrary.MakeTransform` (+ (`self.GetEyeLocation`) (* _returnvalue_2 40.0)) _returnvalue) (* _returnvalue_2 (`self.ThrowForce`))))))

(fn `GetWorldAimEndPoint`
  (returns (EndPoint :type "Vector Structure"))
  (locals (StartLoc :type "Vector Structure") (AimRotation :type "Rotator Structure"))
  (bind _startloc (`local.StartLoc`))
  (`|ExecutionSequence`
    (:`then_0`
      ;[1 1 1] Get StartLoc and AimRotation
      (if (`/Game/GenericShooter/Addons/CharacterCameraManager/Core/BP_CharacterCameraManagerComponent.IsInThirdPerson` (`self.BP_CharacterCameraManagerComponent`))
        (bind _desiredview (`CameraComponent.GetCameraView` (`self.ThirdPersonCamera`) 0.0))
        (bind (_location _rotation) (break `MinimalViewInfo` _desiredview))
        (set `local.StartLoc` _location)
        (set `local.AimRotation` _rotation)
        (else
          (set `local.StartLoc` (`self.GetEyeLocation`))
          (set `local.AimRotation` (`self.GetControlRotation`)))))
    (:`then_1`
      ;[1 1 1] Project Aim to get a world point
      (bind _outhit (`KismetSystemLibrary.LineTraceSingle` _startloc (+ _startloc (* (`KismetMathLibrary.Normal` (`KismetMathLibrary.Conv_RotatorToVector` (`local.AimRotation`))) 10000.0)) "TraceTypeQuery1"))
      (bind (_bblockinghit _binitialoverlap _time _distance _location_2 _impactpoint _normal _impactnormal _physmat _hitactor _hitcomponent _hitbonename _hititem _faceindex _tracestart _traceend) (`GameplayStatics.BreakHitResult` _outhit))
      (return (`KismetMathLibrary.SelectVector` _impactpoint _traceend _bblockinghit)))))

(fn `GiveDefaultWeapons`
  (locals (NewDefaultItems :type "Array of /Game/GenericShooter/Addons/WeaponSystem/Core/BP_Weapon_ItemInfo_Base Object Reference"))
  (bind _bp_wicomponent (`self.BP_WIComponent`))
  ;[1 1 1] Only server can spawn weapons
  (`/Engine/EditorBlueprintResources/ActorMacros.Switch Has Authority`
    (:`Authority`
      (`|ExecutionSequence`
        (:`then_0`
          ;[1 1 1] Grant inventory and equip weapon
          (bind _newiteminfo (`/Game/GenericShooter/Addons/SlotInventory/Core/BP_SlotInventoryComponent.AddItemFromItemInfoClass` _bp_wicomponent "/Game/GenericShooter/Addons/WeaponSystem/Examples/Rifle/BP_Weapon_Info_Rifle.BP_Weapon_Info_Rifle_C" false))
          (bind _newiteminfo_2 (`/Game/GenericShooter/Addons/SlotInventory/Core/BP_SlotInventoryComponent.AddItemFromItemInfoClass` _bp_wicomponent "/Game/GenericShooter/Addons/WeaponSystem/Examples/Shotgun/BP_Weapon_Info_Shotgun.BP_Weapon_Info_Shotgun_C" false))
          (bind _newiteminfo_3 (`/Game/GenericShooter/Addons/SlotInventory/Core/BP_SlotInventoryComponent.AddItemFromItemInfoClass` _bp_wicomponent "/Game/GenericShooter/Addons/WeaponSystem/Examples/Pistol/BP_Weapon_ItemInfo_Pistol.BP_Weapon_ItemInfo_Pistol_C" false))
          (bind _newiteminfo_4 (`/Game/GenericShooter/Addons/SlotInventory/Core/BP_SlotInventoryComponent.AddItemFromItemInfoClass` _bp_wicomponent "/Game/GenericShooter/Addons/WeaponSystem/Examples/GrenadeLauncher/BP_Weapon_ItemInfo_GrenadeLauncher.BP_Weapon_ItemInfo_GrenadeLauncher_C" false))
          (bind _newiteminfo_5 (`/Game/GenericShooter/Addons/SlotInventory/Core/BP_SlotInventoryComponent.AddItemFromItemInfoClass` _bp_wicomponent "/Game/GenericShooter/Addons/WeaponSystem/Examples/RocketLauncher/BP_Weapon_Info_RocketLauncher.BP_Weapon_Info_RocketLauncher_C" true))
          (set `/Game/GenericShooter/Addons/SlotInventory/Core/BP_SlotInventoryComponent.GameplayActiveItem` _newiteminfo _bp_wicomponent)
          (set `self.DesiredWeaponInfo` (cast `/Game/GenericShooter/Addons/WeaponSystem/Core/BP_Weapon_ItemInfo_Base` _newiteminfo :!pure true))
          (`self.SpawnAndEquipDesiredWeapon`))
        (:`then_1`
          ;[1 1 1] Tell item infos about their owner's reserve ammo for UI purposes
          (for _array_element (`|MakeArray` (cast `/Game/GenericShooter/Addons/WeaponSystem/Core/BP_Weapon_ItemInfo_Base` _newiteminfo_3 :!pure true) (cast `/Game/GenericShooter/Addons/WeaponSystem/Core/BP_Weapon_ItemInfo_Base` _newiteminfo :!pure true) (cast `/Game/GenericShooter/Addons/WeaponSystem/Core/BP_Weapon_ItemInfo_Base` _newiteminfo_2 :!pure true) (cast `/Game/GenericShooter/Addons/WeaponSystem/Core/BP_Weapon_ItemInfo_Base` _newiteminfo_4 :!pure true) (cast `/Game/GenericShooter/Addons/WeaponSystem/Core/BP_Weapon_ItemInfo_Base` _newiteminfo_5 :!pure true))
            (set `/Game/GenericShooter/Addons/WeaponSystem/Core/BP_Weapon_ItemInfo_Base.ReserveAmmoStorageAsObject` (`self.BP_AmmoStorageComponent`) _array_element)))))
    (:`Remote`
      (return))))

(fn `IsAlive`
  (returns (Alive :type Boolean))
  (return (`/Game/GenericShooter/Addons/HealthComponent/Core/BP_HealthComponent.IsAlive` (`self.BP_HealthComponent`))))

(fn `NotifyCharacterWeaponManagerWidgetBlueprintIsReady`
  (returns (bNotified :type Boolean))
  (`/Game/GenericShooter/Addons/WeaponSystem/Core/BP_CharacterWeaponManagementComponent.RebuildUI` (`self.BP_CharacterWeaponManagementComponent`))
  (return false))

(fn `NotifyInstigatedDamage`
  (params (Damage :type "Float (double-precision)") (DamageType :type "DamageType Class Reference") (DamagedActor :type "Actor Object Reference") (DamageCauser :type "Actor Object Reference"))
  (returns (bNotified :type Boolean))
  (`/Game/GenericShooter/Addons/WeaponSystem/Core/BP_CharacterWeaponManagementComponent.NotifyInstigatedDamage` (`self.BP_CharacterWeaponManagementComponent`) Damage DamageType DamagedActor DamageCauser)
  (return true))

(fn `OnHolsterFinished`
  (`self.DebugPrintWeaponLogic` "OnHolsterFinished"
    (:`Out`
      (set `/Game/GenericShooter/Addons/SlotInventory/Core/BP_SlotInventoryComponent.GameplayActiveItem` null (`self.BP_WIComponent`))
      (`/Engine/EditorBlueprintResources/ActorMacros.Switch Has Authority`
        (:`Authority`
          (`self.SpawnAndEquipDesiredWeapon`)
          (return))
        (:`Remote`
          (return))))))

(fn `OnItemInfoSelected`
  (params (SelectedItemInfo :type "/Game/GenericShooter/Addons/Common/Blueprints/BaseClasses/BP_SlotInventory_ItemInfo_Base Object Reference"))
  (bind _bp_characterweaponmanagementcomponent (`self.BP_CharacterWeaponManagementComponent`))
  (bind _asbp_weapon_item_info_base (cast `/Game/GenericShooter/Addons/WeaponSystem/Core/BP_Weapon_ItemInfo_Base` SelectedItemInfo)
    (:`then`
      (if (!= _asbp_weapon_item_info_base (`/Game/GenericShooter/Addons/SlotInventory/Core/BP_SlotInventoryComponent.GameplayActiveItem` (`self.BP_WIComponent`)))
        (bind _output_get (set `self.DesiredWeaponInfo` _asbp_weapon_item_info_base))
        (`/Engine/EditorBlueprintResources/ActorMacros.Switch Has Authority`
          (:`Authority`
            _)
          (:`Remote`
            (`self.ServerSwitchToWeapon` _output_get)))
        (`/Game/GenericShooter/Addons/WeaponSystem/Core/BP_CharacterWeaponManagementComponent.Weapon` _bp_characterweaponmanagementcomponent
          (:`then`
            (`/Game/GenericShooter/Addons/WeaponSystem/Core/BP_CharacterWeaponManagementComponent.HolsterWeapon` _bp_characterweaponmanagementcomponent false)
            (return))
          (:`else`
            (`/Engine/EditorBlueprintResources/ActorMacros.Switch Has Authority`
              (:`Authority`
                (`self.DebugPrintWeaponLogic` "Not holding a weapon, performing fast equip."
                  (:`Out`
                    (`self.SpawnAndEquipDesiredWeapon`)
                    (return))))
              (:`Remote`
                (return)))))
        (else
          (`self.DebugPrintWeaponLogic` "Selected Item same as current item."
            (:`Out`
              (return))))))
    (:`CastFailed`
      (`self.DebugPrintWeaponLogic` "Selected Item not a valid Weapon Info class."
        (:`Out`
          (return))))))

(fn `OnTeamNumChanged`
  (params (NewTeamNum :type Byte))
  (`self.UpdateSkinnerParameters`)
  (return))

(fn `RequestTeamChange`
  (params (DesiredTeamIndex :type Integer))
  (returns (bRequested :type Boolean))
  (bind _brequested (message `/Game/GenericShooter/Addons/Common/Blueprints/Interfaces/BPI_TeamMember.RequestTeamChange` (`self.PlayerState`) DesiredTeamIndex))
  (return _brequested))

(fn `SetTeamNumIfServer`
  (params (TeamNum :type Byte))
  (returns (NewTeamNum :type Byte))
  (bind _newteamnum (message `/Game/GenericShooter/Addons/Common/Blueprints/Interfaces/BPI_TeamMember.SetTeamNumIfServer` (`self.PlayerState`) TeamNum))
  (return _newteamnum))

(fn `SetUpNetworkingBehavior`
  (bind _firstpersonarms (`self.FirstPersonArms`))
  (bind _returnvalue (or (`KismetSystemLibrary.IsServer`) (`KismetSystemLibrary.IsDedicatedServer`)))
  (`|ExecutionSequence`
    (:`then_0`
      (set `SkinnedMeshComponent.bEnableUpdateRateOptimizations` (not _returnvalue) _firstpersonarms)
      (set `SkinnedMeshComponent.MeshComponentUpdateFlag` (select `bool` _returnvalue :`false` "OnlyTickPoseWhenRendered" :`true` "AlwaysTickPoseAndRefreshBones" :!type "EMeshComponentUpdateFlag Enum") _firstpersonarms)
      (return))
    (:`then_1`
      (bind _playerstate (`self.PlayerState`)
        (:`then`
          (add `/Game/GenericShooter/Addons/TeamManager/Core/BP_TeamMemberComponent.OnTeamNumChanged` (`self.GetComponentByClass` _playerstate "/Game/GenericShooter/Addons/TeamManager/Core/BP_TeamMemberComponent.BP_TeamMemberComponent_C") (`|CreateDelegate` :!event `OnTeamNumChanged`))
          (return))
        (:`else`
          (`KismetSystemLibrary.PrintString` "Fuck")
          (return))))))

(fn `SpawnAndEquipDesiredWeapon`
  (bind _desiredweaponinfo (`self.DesiredWeaponInfo`)
    (:`then`
      (set `/Game/GenericShooter/Addons/WeaponSystem/Core/BP_Weapon_ItemInfo_Base.ReserveAmmoStorageAsObject` (`self.BP_AmmoStorageComponent`) _desiredweaponinfo)
      (bind _newactor (`/Game/GenericShooter/Addons/Common/Blueprints/BaseClasses/BP_SlotInventory_ItemInfo_Base.SpawnActor` _desiredweaponinfo self self false))
      (`/Game/GenericShooter/Addons/WeaponSystem/Core/BP_CharacterWeaponManagementComponent.ServerEquipWeapon` (`self.BP_CharacterWeaponManagementComponent`) (cast `/Game/GenericShooter/Addons/WeaponSystem/Core/BP_Weapon_Base` _newactor :!pure true) (`self.BP_AmmoStorageComponent`))
      (set `/Game/GenericShooter/Addons/SlotInventory/Core/BP_SlotInventoryComponent.GameplayActiveItem` (`self.DesiredWeaponInfo`) (`self.BP_WIComponent`))
      (set `self.DesiredWeaponInfo` null)
      (return))
    (:`else`
      (`KismetSystemLibrary.PrintString` "ERROR: Server called SpawnAndEquipDesiredWeapon but Desired Weapon Info is not valid!")
      (return))))

(fn `UpdateMesh`
  (locals (InvalidIDMessage :type String :default "UPDATE MESH CALLED WITH INVALID CHARACTER ID"))
  (`/Game/GenericShooter/Addons/WeaponSystem/Core/BP_CharacterWeaponManagementComponent.LoadAllIdlesAndAimOffsets` (`self.BP_CharacterWeaponManagementComponent`))
  (return))

(fn `UpdateSkinnerParameters`
  (bind _teamnum (`self.GetTeamNum`))
  (`/Game/GenericShooter/Addons/Skinner/Core/BP_SkinnerComponent.SetMaterialScalarParameter` (`self.BP_BasicSkinnerComponent`) (`self.TeamNumMatParameterName`) (`KismetMathLibrary.Conv_ByteToDouble` _teamnum) false)
  (return))

(fn `UserConstructionScript`
  (`parent.UserConstructionScript`))