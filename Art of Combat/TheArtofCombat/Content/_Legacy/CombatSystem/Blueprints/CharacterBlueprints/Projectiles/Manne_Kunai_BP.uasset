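; Kunai projectile actor in the legacy combat system that damages guard AI characters on overlap.
; Tick-driven delays switch on the collision capsule shortly after spawn and destroy the actor after a timeout.
; Overlapping an AI_Guard_BP child multicasts a hit emitter, then a server event applies random ranged damage and sends the victim a projectile-hit message.
; The projectile destroys itself after the hit and ignores other actor classes.
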(event `self.ReceiveTick`
  (params (DeltaSeconds :type "Float (single-precision)"))
  (`KismetSystemLibrary.Delay` 0.2)
  (`PrimitiveComponent.SetCollisionEnabled` (`self.Collision Capsule`) "QueryAndPhysics")
  (`KismetSystemLibrary.Delay` 10.0)
  (`self.K2_DestroyActor`))

(event `On Begin Overlap With EC`
  (params (`Other Actor` :type "Actor Object Reference") (`Other Comp` :type "PrimitiveComponent Object Reference") (`Other Body Index` :type Integer) (`From Sweep` :type Boolean) (`Sweep Result` :type "HitResult Structure"))
  ;[0.6059 0.6434 1] On Begin Overlap with EC
  (if (`KismetMathLibrary.ClassIsChildOf` (`GameplayStatics.GetObjectClass` `Other Actor`) "/Game/_Legacy/CombatSystem/Blueprints/CharacterBlueprints/AI/_Parent/AI_Guard_BP.AI_Guard_BP_C")
    (`self.Emitter Spawn`)
    (`KismetSystemLibrary.Delay` 0.05)
    (`self.Deal Damage` `Other Actor`)
    (`self.K2_DestroyActor`)))

(event `self.Collision Capsule.OnComponentBeginOverlap`
  (params (OverlappedComponent :type "PrimitiveComponent Object Reference") (OtherActor :type "Actor Object Reference") (OtherComp :type "PrimitiveComponent Object Reference") (OtherBodyIndex :type Integer) (bFromSweep :type Boolean) (SweepResult :type "HitResult Structure (by ref)"))
  ;[0 0 0] On Component Begin Overlap (Collision Capsule)
  (`self.On Begin Overlap With EC` OtherActor OtherComp OtherBodyIndex bFromSweep SweepResult))

(event `Emitter Spawn`
  ;[0 0 0] Emitter Spawn - Multicast to all Relevant Clients
  (`GameplayStatics.SpawnEmitterAtLocation` "/Game/_Legacy/CombatSystem/Particles/P_Kunai_Hit.P_Kunai_Hit" (`SceneComponent.K2_GetComponentLocation` (`self.Collision Capsule`))))

(event `Deal Damage`
  (params (`Damaged Actor` :type "Actor Object Reference"))
  ;[0.8926 1 0.3959] Deal Damage - Run on Server
  (`GameplayStatics.ApplyDamage` `Damaged Actor` (`KismetMathLibrary.RandomFloatInRange` (`self.Min Damage`) (`self.Max Damage`)))
  (message `/Game/_Legacy/CombatSystem/Blueprints/BlueprintInterface/Menu_Manne_AI_Interface_.Projectile Hit EC` `Damaged Actor`))

(fn `UserConstructionScript`)