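; Kunai projectile that damages characters of a configurable class on overlap and self-destroys after its lifespan.
; Collision turns on after a delay; a hit spawns an impact emitter, then for Manne_BP targets plays surface-based sounds, notifies them and applies delayed random damage before destruction.
; It records the first non-parry component struck on a Manne_BP, flagging head bullseyes.
; Deflection redirects velocity using the supplied vector and suppresses further hit handling.
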(event `self.ReceiveBeginPlay`
  (`KismetSystemLibrary.Delay` (`self.Life Span`))
  (`/Engine/EditorBlueprintResources/StandardMacros.IsValid` self
    (:`Is Valid`
      (`self.K2_DestroyActor`))))

(event `self.ReceiveTick`
  (params (DeltaSeconds :type "Float (single-precision)"))
  (`KismetSystemLibrary.Delay` (`self.Delay Before Enabling Collision`))
  (`PrimitiveComponent.SetCollisionEnabled` (`self.Collision Capsule`) "QueryAndPhysics"))

(event `self.Collision Capsule.OnComponentBeginOverlap`
  (params (OverlappedComponent :type "PrimitiveComponent Object Reference") (OtherActor :type "Actor Object Reference") (OtherComp :type "PrimitiveComponent Object Reference") (OtherBodyIndex :type Integer) (bFromSweep :type Boolean) (SweepResult :type "HitResult Structure (by ref)"))
  ;[0.6059 0.6434 1] On Begin Overlap with EC
  (if (`KismetMathLibrary.ClassIsChildOf` (`GameplayStatics.GetObjectClass` OtherActor) (`self.Parent Class To Check For Collision Against`))
    (if (not (`self.IsBeingDeflected?`))
      (`self.Get First Overlapped Component On Hit Actor` OtherComp OtherActor)
      (bind _returnvalue (`GameplayStatics.SpawnEmitterAtLocation` (`self.Emitter To Spawn At Point of Impact`) (- (`SceneComponent.K2_GetComponentLocation` (`self.Collision Capsule`)) (`self.Emitter Spawn Location Modifier`)) (`self.Emitter Spawn Rotation`)))
      (`/Engine/EditorBlueprintResources/StandardMacros.IsValid` _returnvalue
        (:`Is Valid`
          (`SceneComponent.SetWorldScale3D` _returnvalue (`self.Emitter Scale`)))
        (:`Is Not Valid`
          _))
      (bind _asmanne_bp (cast `/Game/_ADNeo/CombatSys/BPs/CharBPs/Manne/_Parent/Manne_BP` OtherActor))
      (`/Engine/EditorBlueprintResources/StandardMacros.IsValid` _asmanne_bp
        (:`Is Valid`
          (`/Game/_ADNeo/CombatSys/BPs/CharBPs/Manne/_Parent/Manne_BP.Play Hit Sounds` _asmanne_bp (`MaterialInterface.GetPhysicalMaterial` (`PrimitiveComponent.GetMaterial` (`Character.Mesh` _asmanne_bp) 0))))
        (:`Is Not Valid`
          _))
      (`/Engine/EditorBlueprintResources/StandardMacros.IsValid` OtherActor
        (:`Is Valid`
          (message `/Game/_ADNeo/CombatSys/BPs/Misc/Interfaces/Projectile_Interface.Kunai Hit TC` OtherActor))
        (:`Is Not Valid`
          _))
      (`KismetSystemLibrary.Delay` (`self.Delay Duration Before Dealing Damage After Successful Hit`))
      (`/Engine/EditorBlueprintResources/StandardMacros.IsValid` OtherActor
        (:`Is Valid`
          (`self.Deal Damage` OtherActor))
        (:`Is Not Valid`
          _))
      (`KismetSystemLibrary.Delay` (`self.Delay Duration Before Destruction After Successful Hit`))
      (`self.K2_DestroyActor`))))

(event `Deal Damage`
  (params (`Hit Actor` :type "Actor Object Reference"))
  ;[0.8926 1 0.3959] Deal Damage
  (`GameplayStatics.ApplyDamage` `Hit Actor` (`KismetMathLibrary.RandomFloatInRange` (`self.Min Dmg`) (`self.Max Dmg`)) (`self.GetInstigatorController`) self))

(event `Deflect Projectile`
  (params (Character :type "Character Object Reference") (`Impact Location` :type "Vector Structure"))
  ;[0 0 0] Deflect Projectile
  (`self.Exec_Deflect Projectile` Character `Impact Location`))

(event `Exec_Deflect Projectile`
  (params (Character :type "Character Object Reference") (`Impact Location` :type "Vector Structure"))
  ;[0 0 0] Deflect Projectile
  (set `self.IsBeingDeflected?` true)
  (set `MovementComponent.Velocity` `Impact Location` (`self.ProjectileMovement`)))

(event `Get First Overlapped Component On Hit Actor`
  (params (`Other Comp` :type "PrimitiveComponent Object Reference") (`Other Actor` :type "Actor Object Reference"))
  ;[0 0 0] Get First Overlapped Component On Hit Actor
  (bind _asmanne_bp (cast `/Game/_ADNeo/CombatSys/BPs/CharBPs/Manne/_Parent/Manne_BP` `Other Actor`))
  (if (== (`/Game/_ADNeo/CombatSys/BPs/CharBPs/Manne/_Parent/Manne_BP.CollisionCapsuleForParry` _asmanne_bp) `Other Comp`)
    _
    (elif (not (== (`/Game/_ADNeo/CombatSys/BPs/CharBPs/Manne/_Parent/Manne_BP.ParryCapsule` _asmanne_bp) `Other Comp`))
      (`/Engine/EditorBlueprintResources/StandardMacros.DoOnce` false
        (:`Completed`
          (bind _output_get (set `self.Component For Bullseye` `Other Comp`))
          (if (== _output_get (`/Game/_ADNeo/CombatSys/BPs/CharBPs/Manne/_Parent/Manne_BP.DmgRcvCapsule_Head` _asmanne_bp))
            (set `self.Bullseye_Current` (`self.Bullseye_Head`))))))))

(fn `UserConstructionScript`)