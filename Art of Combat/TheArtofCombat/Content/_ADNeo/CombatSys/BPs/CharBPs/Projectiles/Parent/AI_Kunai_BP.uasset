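; AI kunai projectile Blueprint, a parent class that damages targets of a configurable class on overlap.
; Tick enables capsule collision after a short delay, then destroys the actor after a configurable lifetime.
; A valid overlap spawns an impact emitter, sends KunaiHitTCMessage to the target, then briefly waits before applying random damage within a range and destroying itself.
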(event `self.ReceiveTick`
  (params (DeltaSeconds :type "Float (single-precision)"))
  (`KismetSystemLibrary.Delay` 0.2)
  (`PrimitiveComponent.SetCollisionEnabled` (`self.Collision Capsule`) "QueryAndPhysics")
  (`KismetSystemLibrary.Delay` (`self.Delay Duration Before Actor Destruction`))
  (`self.K2_DestroyActor`))

(event `self.Collision Capsule.OnComponentBeginOverlap`
  (params (OverlappedComponent :type "PrimitiveComponent Object Reference") (OtherActor :type "Actor Object Reference") (OtherComp :type "PrimitiveComponent Object Reference") (OtherBodyIndex :type Integer) (bFromSweep :type Boolean) (SweepResult :type "HitResult Structure (by ref)"))
  ;[0.6059 0.6434 1] On Begin Overlap with TC
  (if (`KismetMathLibrary.ClassIsChildOf` (`GameplayStatics.GetObjectClass` OtherActor) (`self.Parent Class To Check For Collision Against`))
    (`GameplayStatics.SpawnEmitterAtLocation` (`self.Emitter To Spawn At Point of Impact`) (`SceneComponent.K2_GetComponentLocation` (`self.Collision Capsule`)) (struct))
    (message `/Game/_ADNeo/CombatSys/BPs/Misc/Interfaces/Projectile_Interface.Kunai Hit TC` OtherActor)
    (`KismetSystemLibrary.Delay` 0.05)
    (`self.Deal Damage` OtherActor)
    (`self.K2_DestroyActor`)))

(event `Deal Damage`
  (params (`Hit Actor` :type "Actor Object Reference"))
  ;[0.8926 1 0.3959] Deal Damage
  (`GameplayStatics.ApplyDamage` `Hit Actor` (`KismetMathLibrary.RandomFloatInRange` (`self.Min Dmg`) (`self.Max Dmg`)) null self))

(fn `UserConstructionScript`)